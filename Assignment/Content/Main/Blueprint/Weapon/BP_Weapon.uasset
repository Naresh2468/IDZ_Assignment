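; BP_Weapon is a world weapon actor with an interaction prompt.
; Its construction script sets the static mesh from the data table row referenced by its Weapon item.
; On BeginPlay it passes the weapon name to the UMG_Interact widget, which the box overlap shows or hides for player character 0.
; InteractObject only hides the actor and disables mesh collision, with no inventory logic here.
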(event `self.ReceiveBeginPlay`
  (bind _asumg_interact (cast `/Game/Main/Blueprint/UI/Object/UMG_Interact` (`WidgetComponent.GetWidget` (`self.Widget`))))
  (bind _output_get (set `self.As UMG Interact` _asumg_interact))
  (`/Game/Main/Blueprint/UI/Object/UMG_Interact.Text` _output_get (`self.WeaponName`)))

(event `/Game/Main/Blueprint/Interface/BPI_Interact.InteractObject`
  (`self.SetActorHiddenInGame` true)
  (`PrimitiveComponent.SetCollisionEnabled` (`self.StaticMesh`) "NoCollision"))

(event `self.Box.OnComponentBeginOverlap`
  (params (OverlappedComponent :type "PrimitiveComponent Object Reference") (OtherActor :type "Actor Object Reference") (OtherComp :type "PrimitiveComponent Object Reference") (OtherBodyIndex :type Integer) (bFromSweep :type Boolean) (SweepResult :type "HitResult Structure (by ref)"))
  (if (== OtherActor (`GameplayStatics.GetPlayerCharacter` 0))
    (`self.F_ShowandHide` true)))

(event `self.Box.OnComponentEndOverlap`
  (params (OverlappedComponent :type "PrimitiveComponent Object Reference") (OtherActor :type "Actor Object Reference") (OtherComp :type "PrimitiveComponent Object Reference") (OtherBodyIndex :type Integer))
  (if (== OtherActor (`GameplayStatics.GetPlayerCharacter` 0))
    (`self.F_ShowandHide` false)))

(fn `F_ShowandHide`
  (params (Visibility :type Boolean))
  (`SceneComponent.SetVisibility` (`self.Widget`) Visibility false))

(fn `UserConstructionScript`
  (bind _weapon (`self.Weapon`))
  (bind _returnvalue (`|GetDataTableRow` (break `DataTableRowHandle` (break `/Game/Main/Blueprint/Framework/Data/WeaponSlots` _weapon)) (`.RowName` (break `DataTableRowHandle` (break `/Game/Main/Blueprint/Framework/Data/WeaponSlots` _weapon))))
    (:`then`
      (`StaticMeshComponent.SetStaticMesh` (`self.StaticMesh`) (`.WeaponMesh_4_C20199EA46794543BE4D32A5B5AA674C` (break `/Game/Main/Blueprint/Framework/Data/WeaponInfo` _returnvalue))))))