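; Main player character that handles melee attack input, interaction, pausing, health and death.
; Attack and weapon inputs go to BPCAttack, while interacting through BPI_Interact reveals the sword and sets CanEquipped.
; Damage updates the health bar via the cached GM_GameManager; death triggers ragdoll, disables input, fades the camera and reloads MainGame.
; Crouch edits a State array, but the movement logic that would apply it is disconnected.
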(event `self.ReceiveBeginPlay`
  ;[0 0 0 0.5] Player Setup
  (`parent.ReceiveBeginPlay`)
  (`self.F_DefaultValue`))

(event `self.ReceiveAnyDamage`
  (params (Damage :type "Float (single-precision)") (DamageType :type "DamageType Object Reference") (InstigatedBy :type "Controller Object Reference") (DamageCauser :type "Actor Object Reference"))
  (`self.F_Damage` Damage))

(event `EnhancedInput|/Game/Main/Blueprint/InputData/Inputs/IA_MeleeAttack`
  (params (ActionValue :type Boolean) (ElapsedSeconds :type "Float (double-precision)") (TriggeredSeconds :type "Float (double-precision)") (InputAction :type "InputAction Object Reference" :default "/Game/Main/Blueprint/InputData/Inputs/IA_MeleeAttack.IA_MeleeAttack"))
  ; Action
  (:`Triggered`
    (`/Game/Main/Blueprint/Character/MainPlayer/Component/BPC_Attack.SwordAttack` (`self.BPC_Attack`))))

(event `EnhancedInput|/Game/Main/Blueprint/InputData/Inputs/IA_PrimaryWeapon`
  (params (ActionValue :type Boolean) (ElapsedSeconds :type "Float (double-precision)") (TriggeredSeconds :type "Float (double-precision)") (InputAction :type "InputAction Object Reference" :default "/Game/Main/Blueprint/InputData/Inputs/IA_PrimaryWeapon.IA_PrimaryWeapon"))
  ; Action
  (:`Triggered`
    (`/Game/Main/Blueprint/Character/MainPlayer/Component/BPC_Attack.F_EquippedWeapon` (`self.BPC_Attack`))))

(event `Respawn`
  (`PlayerCameraManager.StartCameraFade` :`self` (`GameplayStatics.GetPlayerCameraManager` 0) :`ToAlpha` 1.0 :`Duration` 2.5 :`bHoldWhenFinished` true)
  (`KismetSystemLibrary.Delay` 3.0)
  (`GameplayStatics.OpenLevelBySoftObjectPtr` "/Game/Main/Map/MainGame.MainGame"))

(event `self.F_InteractObjects`
  (params (result :type "Actor Object Reference"))
  ; Action
  (`self.F_InteractMessage` result))

(event `EnhancedInput|/Game/Main/Blueprint/InputData/Inputs/IA_GamePause`
  (params (ActionValue :type Boolean) (ElapsedSeconds :type "Float (double-precision)") (TriggeredSeconds :type "Float (double-precision)") (InputAction :type "InputAction Object Reference" :default "/Game/Main/Blueprint/InputData/Inputs/IA_GamePause.IA_GamePause"))
  ; Action
  (:`Triggered`
    (`/Game/Main/Blueprint/Framework/Gamemode/GM_GameManager.PauseGame` (`self.As GM Game Manager`))))

(fn `F_Crouch`
  (params (Condition :type Boolean))
  (bind _state (`self.State`))
  (if Condition
    (`KismetArrayLibrary.Array_Set` _state (+ (`KismetArrayLibrary.Array_LastIndex` _state) 1) "NewEnumerator3" true)
    (`self.F_MovementBp` :!label _label)
    (elif (`KismetArrayLibrary.Array_Contains` (`self.State`) "NewEnumerator3")
      (`KismetArrayLibrary.Array_RemoveItem` (`self.State`) "NewEnumerator3")
      (goto _label))))

(fn `F_Damage`
  (params (Damage :type "Float (double-precision)"))
  (bind _uiref (`/Game/Main/Blueprint/Framework/Gamemode/GM_GameManager.UIRef` (`self.As GM Game Manager`)))
  (bind _output_get (set `self.Health` (- (`self.Health`) Damage)))
  (if (<= _output_get 0.0)
    (`/Game/Main/Blueprint/UI/UMG_Main.HealthBar` _uiref 0.0)
    (`self.DisableInput` (`GameplayStatics.GetPlayerController` 0))
    (`PrimitiveComponent.SetSimulatePhysics` (`self.Mesh`) true)
    (`self.Respawn`)
    (`PrimitiveComponent.SetCollisionEnabled` (`self.CapsuleComponent`) "NoCollision")
    (else
      (`/Game/Main/Blueprint/UI/UMG_Main.HealthBar` _uiref (`self.Health`)))))

(fn `F_DefaultValue`
  (bind _asgm_game_manager (cast `/Game/Main/Blueprint/Framework/Gamemode/GM_GameManager` (`GameplayStatics.GetGameMode`)))
  (set `self.As GM Game Manager` _asgm_game_manager))

(fn `F_InteractMessage`
  (params (Object :type "Object Object Reference"))
  (if (`KismetSystemLibrary.DoesImplementInterface` Object "/Game/Main/Blueprint/Interface/BPI_Interact.BPI_Interact_C")
    (message `/Game/Main/Blueprint/Interface/BPI_Interact.InteractObject` Object)
    (set `self.canEquipped?` true)
    (`SceneComponent.SetVisibility` (`self.Weapon_Sword`) true false)
    (else
      (`KismetSystemLibrary.PrintString` (`KismetSystemLibrary.GetDisplayName` Object)))))

(fn `F_MovementBp`)

(fn `PlayerRef`
  (returns (BP_Player :type "/Game/Main/Blueprint/Character/MainPlayer/BP_Player Object Reference"))
  (return self))

(fn `UserConstructionScript`)