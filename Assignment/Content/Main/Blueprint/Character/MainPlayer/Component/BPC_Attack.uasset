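; Player attack component that handles equipping or holstering the sword and melee combat.
; Attacks play random montages, queue one follow-up input for combos, and use a timer to turn the player toward control rotation.
; A looping timer sphere-traces between two blade points, applying damage, camera shake, sound and particles to "Damageable" actors, with DoOnce gates throttling repeat hits.
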(event `Equiped Weapon`
  (bind _isweaponequiped_ (`self.isWeaponEquiped?`))
  (bind _bp_playerref (`self.BP PlayerRef`))
  (bind _output_get (set `self.isWeaponEquiped?` (not _isweaponequiped_)))
  (if _isweaponequiped_
    _
    (else
      _))
  (`SceneComponent.K2_AttachToComponent` (`/Game/Main/Blueprint/Character/MainPlayer/BP_Player.Weapon_Sword` _bp_playerref) (`Character.Mesh` _bp_playerref) (select `bool` _output_get :`false` (`self.WeaponHolster`) :`true` (`self.WeaponEquiped`)) "KeepRelative" "KeepRelative" "KeepRelative" true))

(event `self.ReceiveBeginPlay`
  (bind _bp_player (message `/Game/Main/Blueprint/Interface/BPI_Communication.PlayerRef` (`self.GetOwner`)))
  (set `self.BP PlayerRef` _bp_player))

(event `SwordAttack`
  (if (and (not (`|EnumEquality` (`|GetArrayItem` (`/Game/Main/Blueprint/Character/MainPlayer/BP_Player.State` (`self.BP PlayerRef`))) "NewEnumerator3")) (`self.isWeaponEquiped?`))
    (`self.SwordAttackStart`)
    (`self.CE_RotateToward`)
    (`KismetSystemLibrary.Delay` 0.3)
    (`KismetSystemLibrary.K2_ClearAndInvalidateTimerHandle` (`self.RotationAttack`))))

(event `CE_RotateToward`
  (bind _returnvalue (`KismetSystemLibrary.K2_SetTimerDelegate` (`|CreateDelegate` :!event `Rotate`) 0.002 true))
  (set `self.RotationAttack` _returnvalue))

(event `Rotate`
  (bind _bp_playerref (`self.BP PlayerRef`))
  (bind _returnvalue (`Actor.K2_GetActorRotation` _bp_playerref))
  (bind (_returnvalue_roll _returnvalue_pitch _returnvalue_yaw) (`KismetMathLibrary.BreakRotator` (`KismetMathLibrary.RInterpTo` _returnvalue (`Pawn.GetControlRotation` _bp_playerref) 0.002 (`self.RotationSpeed`))))
  (`Actor.K2_SetActorRotation` _bp_playerref (`KismetMathLibrary.MakeRotator` (.roll _returnvalue) (.pitch _returnvalue) _returnvalue_yaw) false))

(event `SwordAttackStart`
  (bind _returnvalue (`KismetMathLibrary.RandomIntegerInRange` 0 (`KismetArrayLibrary.Array_LastIndex` (`self.AttackM`))))
  (if (`self.bisAttacking?`)
    (set `self.SaveAttack` true)
    (else
      (set `self.bisAttacking?` true)
      (`/Engine/EditorBlueprintResources/StandardMacros.DoOnce` false :!label _label
        (:`Completed`
          (`KismetSystemLibrary.Delay` (`self.DelayGap`))
          (`|PlayMontage` (`Character.Mesh` (`self.BP PlayerRef`)) (`|GetArrayItem` (`self.AttackM`) _returnvalue) 1.25
            (:`then`
              (set `self.Attackindex` (+ _returnvalue 1))
              (goto _label :!via `Reset`))))))))

(event `SwordAtackCombo`
  (if (`self.SaveAttack`)
    (set `self.SaveAttack` false)
    (goto _label)
    (else
      (`self.F_StopFunction`))))

(event `StartSwordTrace`
  (if (`KismetSystemLibrary.K2_IsValidTimerHandle` (`self.SowrdTraceTimer`))
    (`self.SwordTraceStop`))
  (bind _returnvalue (`KismetSystemLibrary.K2_SetTimerDelegate` (`|CreateDelegate` :!event `SwordTraceLoop`) 0.009 true))
  (set `self.SowrdTraceTimer` _returnvalue))

(event `SwordTraceLoop`
  (bind _bp_playerref (`self.BP PlayerRef`))
  (bind (_outhit _returnvalue) (`KismetSystemLibrary.SphereTraceSingle` :`Start` (`SceneComponent.K2_GetComponentLocation` (`/Game/Main/Blueprint/Character/MainPlayer/BP_Player.TopPoint` _bp_playerref)) :`End` (`SceneComponent.K2_GetComponentLocation` (`/Game/Main/Blueprint/Character/MainPlayer/BP_Player.EndPoint` _bp_playerref)) :`Radius` 10.0 :`TraceChannel` "TraceTypeQuery1" :`DrawDebugType` "ForDuration" :`TraceColor` (struct :`R` 1.0 :`G` 0.211286 :`B` 0.951492 :`A` 1.0) :`DrawTime` 0.2))
  (if _returnvalue
    (bind (_bblockinghit _binitialoverlap _time _distance _location _impactpoint _normal _impactnormal _physmat _hitactor) (`GameplayStatics.BreakHitResult` _outhit))
    (if (`Actor.ActorHasTag` _hitactor "Damageable")
      (`/Engine/EditorBlueprintResources/StandardMacros.DoOnce` false :!label _label_2
        (:`Completed`
          (`GameplayStatics.ApplyDamage` _hitactor 10.0)
          (`self.CameraShakeHit` _location)
          (`self.SwordHitSound`)
          (`GameplayStatics.SpawnEmitterAtLocation` null _location (`KismetMathLibrary.MakeRotFromXY` _normal _normal) (`KismetArrayLibrary.Array_Random` (`|MakeArray` (0.5 0.5 0.5) (0.6 0.6 0.6) (0.4 0.4 0.4) :!type "Vector Structure")))
          (`KismetSystemLibrary.PrintString` (`KismetSystemLibrary.GetDisplayName` _hitactor))
          (`|ExecutionSequence`
            (:`then_0`
              (`KismetSystemLibrary.Delay` 0.5)
              (goto _label_2 :!via `Reset`))
            (:`then_1`
              (if (`KismetSystemLibrary.DoesImplementInterface` _hitactor)
                _)))))
      (else
        (`/Engine/EditorBlueprintResources/StandardMacros.DoOnce` false :!label _label_3
          (:`Completed`
            (`GameplayStatics.PlaySoundAtLocation` null (`Actor.K2_GetActorLocation` (`self.BP PlayerRef`)) (struct) 1.0 1.0 0.0 null null null null)))))))

(event `ResetSoundHit`
  (goto _label_3 :!via `Reset`))

(event `Stop Sword trace`
  (`self.SwordTraceStop`))

(event `CameraShakeHit`
  (params (Epicenter :type "Vector Structure"))
  (`GameplayStatics.PlayWorldCameraShake` null Epicenter 0.0 2000.0))

(event `SwordHitSound`
  (`GameplayStatics.PlaySoundAtLocation` null (`Actor.K2_GetActorLocation` (`self.BP PlayerRef`)) (struct) 1.0 1.0 0.0 null null null null))

(fn `F_StopFunction`
  (set `self.bisAttacking?` false)
  (set `self.Attackindex` 0))

(fn `SwordTraceStop`
  (`KismetSystemLibrary.K2_ClearAndInvalidateTimerHandle` (`self.SowrdTraceTimer`))
  (`self.ResetSoundHit`))