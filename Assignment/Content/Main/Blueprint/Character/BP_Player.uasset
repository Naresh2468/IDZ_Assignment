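; Player character Blueprint that handles walking, sprinting and crouching through Enhanced Input actions.
; A State array works as a stack: inputs append or remove Running and Crouch, with sprint blocked while crouched.
; FMovement reads the last entry to toggle crouch and select MaxWalkSpeed.
; At BeginPlay, the configured MaxWalkSpeed becomes sprint speed and half of it becomes walk speed.
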(event `self.ReceiveBeginPlay`
  (`parent.ReceiveBeginPlay`)
  (`self.F_DefaultValue`))

(event `EnhancedInput|/Game/Main/Blueprint/InputData/Inputs/IA_PlayerSprint`
  (params (ActionValue :type Boolean) (ElapsedSeconds :type "Float (double-precision)") (TriggeredSeconds :type "Float (double-precision)") (InputAction :type "InputAction Object Reference" :default "/Game/Main/Blueprint/InputData/Inputs/IA_PlayerSprint.IA_PlayerSprint"))
  (bind _state (`self.State`))
  (:`Triggered`
    (if (and ActionValue (not (`KismetArrayLibrary.Array_Contains` (`self.State`) "NewEnumerator3")))
      (`KismetArrayLibrary.Array_Set` _state (+ (`KismetArrayLibrary.Array_LastIndex` _state) 1) "NewEnumerator2" true)
      (else
        (`KismetArrayLibrary.Array_RemoveItem` (`self.State`) "NewEnumerator2")))
    (`self.F_Movement`)))

(event `EnhancedInput|/Game/Main/Blueprint/InputData/Inputs/IA_PlayerCrouch`
  (params (ActionValue :type Boolean) (ElapsedSeconds :type "Float (double-precision)") (TriggeredSeconds :type "Float (double-precision)") (InputAction :type "InputAction Object Reference" :default "/Game/Main/Blueprint/InputData/Inputs/IA_PlayerCrouch.IA_PlayerCrouch"))
  (:`Triggered`
    (`self.F_Crouch` ActionValue)))

(fn `F_Crouch`
  (params (Condition :type Boolean))
  (bind _state (`self.State`))
  (if Condition
    (`KismetArrayLibrary.Array_Set` _state (+ (`KismetArrayLibrary.Array_LastIndex` _state) 1) "NewEnumerator3" true)
    (`self.F_Movement`)
    (elif (`KismetArrayLibrary.Array_Contains` (`self.State`) "NewEnumerator3")
      (`KismetArrayLibrary.Array_RemoveItem` (`self.State`) "NewEnumerator3")
      (`self.F_Movement`))))

(fn `F_DefaultValue`
  (bind _charactermovement (`self.CharacterMovement`))
  (bind _maxwalkspeed (`CharacterMovementComponent.MaxWalkSpeed` _charactermovement))
  (set `self.Sprint Speed` _maxwalkspeed)
  (bind _output_get (set `CharacterMovementComponent.MaxWalkSpeed` (/ _maxwalkspeed 2.0) _charactermovement))
  (set `self.WalkSpeed` _output_get))

(fn `F_Movement`
  (bind _state (`self.State`))
  (bind _state_2 (`self.State`))
  (if (`|EnumEquality` (`|GetArrayItem` _state (`KismetArrayLibrary.Array_LastIndex` _state)) "NewEnumerator3")
    (`self.Crouch`)
    (else
      (`self.UnCrouch`)))
  (set `CharacterMovementComponent.MaxWalkSpeed` (select `/Game/Main/Blueprint/Character/PlayerState/E_PlayerState` (`|GetArrayItem` _state_2 (`KismetArrayLibrary.Array_LastIndex` _state_2)) :`NewEnumerator1` (`self.WalkSpeed`) :`NewEnumerator2` (`self.Sprint Speed`) :`NewEnumerator3` (`self.CrouchSpeed`)) (`self.CharacterMovement`)))

(fn `UserConstructionScript`)