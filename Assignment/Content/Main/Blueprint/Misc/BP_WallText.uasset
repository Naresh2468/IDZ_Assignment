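; BP_WallText is a placeable actor that displays configurable text in the world through a TextRender component.
; Its construction script applies the Description, font size, color and horizontal and vertical alignment variables to the component.
; The event graph holds only disabled default nodes, so it adds no runtime behavior.
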(fn `UserConstructionScript`
  (bind _textrender (`self.TextRender`))
  (`TextRenderComponent.K2_SetText` _textrender (`self.Description`))
  (`TextRenderComponent.SetWorldSize` _textrender (`self.FontSize`))
  (`TextRenderComponent.SetTextRenderColor` _textrender (`KismetMathLibrary.LinearColor_ToRGBE` (`self.Color`)))
  (`TextRenderComponent.SetHorizontalAlignment` _textrender (`self.H_Alignment`))
  (`TextRenderComponent.SetVerticalAlignment` _textrender (`self.V_Alignment`)))