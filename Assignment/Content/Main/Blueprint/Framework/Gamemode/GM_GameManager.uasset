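; GM_GameManager is a game mode that owns the main UI and handles pausing the game.
; On BeginPlay it creates the UMG_Main widget, passes itself as a reference and adds it to the viewport.
; Its PauseGame event toggles pause, syncs the mouse cursor, informs the widget, and switches input between Game and UI focused on the widget and Game Only.
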(event `self.ReceiveBeginPlay`
  (`parent.ReceiveBeginPlay`)
  (`self.F_WidgetInitialize`))

(event `PauseGame`
  (`self.F_PauseGame`))

(fn `F_PauseGame`
  (bind _returnvalue (`GameplayStatics.GetPlayerController` 0))
  (bind _returnvalue_2 (`GameplayStatics.IsGamePaused`))
  (bind _uiref (`self.UIRef`))
  (if _returnvalue_2
    (`GameplayStatics.SetGamePaused` false)
    (else
      (`GameplayStatics.SetGamePaused` true)))
  (set `PlayerController.bShowMouseCursor` _returnvalue_2 _returnvalue)
  (`/Game/Main/Blueprint/UI/UMG_Main.PauseGame` _uiref _returnvalue_2)
  (if _returnvalue_2
    (`WidgetBlueprintLibrary.SetInputMode_GameAndUIEx` _returnvalue _uiref)
    (else
      (`WidgetBlueprintLibrary.SetInputMode_GameOnly` _returnvalue))))

(fn `F_WidgetInitialize`
  (bind _returnvalue (`|CreateWidget` "/Game/Main/Blueprint/UI/UMG_Main.UMG_Main_C"))
  (bind _output_get (set `self.UIRef` _returnvalue))
  (set `/Game/Main/Blueprint/UI/UMG_Main.GM_Ref` self _output_get)
  (`UserWidget.AddToViewport` _returnvalue 0))

(fn `UserConstructionScript`)