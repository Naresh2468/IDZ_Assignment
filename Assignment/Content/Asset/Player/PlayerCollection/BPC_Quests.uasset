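; Player quest component that tracks the active quest's objectives, drives its on-screen widget and toggles world markers.
; Enemy-kill and chest-open events mark objectives complete, update the widget and count toward quest completion.
; Completion sets a flag for one of three named quests, with the first two unlocking the third.
; Markers switch by quest name, pointing to the commander or, for Friend in Need, also arming the boss call.
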(event `QuestLoadGame`
  (bind (_activequests_questname _activequests_desrciption _activequests_secondary _activequests_completed _activequests_questsobjective) (break `/Game/Main/BP/GameCollection/GameQuest/S_QuestsDetails` (`self.ActiveQuests`)))
  (if (not (`KismetArrayLibrary.Array_IsEmpty` _activequests_questsobjective))
    (bind _returnvalue (`|CreateWidget` "/Game/Main/BP/Widget/QuestsWidget/WI_QuestsPlayerDisplay.WI_QuestsPlayerDisplay_C" :!label _label))
    (bind _output_get (set `self.CurrentQuests` _returnvalue))
    (`UserWidget.AddToViewport` _output_get 0)
    (`/Game/Main/BP/Widget/QuestsWidget/WI_QuestsPlayerDisplay.VisibilityHideQuests` _output_get true)))

(event `ActiveQuestsDisplay`
  (goto _label))

(event `Set Text Quests  active`
  (bind (_activequests_questname _activequests_desrciption _activequests_secondary _activequests_completed _activequests_questsobjective) (break `/Game/Main/BP/GameCollection/GameQuest/S_QuestsDetails` (`self.ActiveQuests`)))
  (if (not (`KismetArrayLibrary.Array_IsEmpty` _activequests_questsobjective))
    (`KismetSystemLibrary.DelayUntilNextTick`)
    (`/Game/Main/BP/Widget/QuestsWidget/WI_QuestsPlayerDisplay.Info` (`self.CurrentQuests`) (`KismetTextLibrary.Conv_NameToText` _activequests_questname) (`KismetTextLibrary.Conv_NameToText` _activequests_desrciption))))

(event `SetObjective`
  (params (Quests :type "/Game/Main/BP/GameCollection/GameQuest/S_QuestsDetails Structure"))
  (bind (_activequests_questname _activequests_desrciption _activequests_secondary _activequests_completed _activequests_questsobjective) (break `/Game/Main/BP/GameCollection/GameQuest/S_QuestsDetails` (`self.ActiveQuests`)))
  (if (not (`KismetArrayLibrary.Array_IsEmpty` _activequests_questsobjective))
    (`KismetSystemLibrary.DelayUntilNextTick`)
    (`/Game/Main/BP/Widget/QuestsWidget/WI_QuestsPlayerDisplay.FillObjectives` (`self.CurrentQuests`) Quests)
    (`KismetSystemLibrary.Delay` 0.2)
    ;[1 1 1] Marker
    (`self.QuestsMarkermaker` true)))

(event `Eliminate EnemyCheck`
  (params (Actor :type "Actor Object Reference"))
  (bind (_activequests_questname _activequests_desrciption _activequests_secondary _activequests_completed _activequests_questsobjective) (break `/Game/Main/BP/GameCollection/GameQuest/S_QuestsDetails` (`self.ActiveQuests`)))
  (bind (_questname _desrciption _secondary _completed _questsobjective) (break `/Game/Main/BP/GameCollection/GameQuest/S_QuestsDetails` (`self.ActiveQuests`)))
  (for (_array_element _array_index) _activequests_questsobjective
    (bind (_names _completed_2 _actortoeliminate _chesttoopen _eilmimateenemyobjective _ischestobjective) (break `/Game/Main/BP/GameCollection/GameQuest/S_QuestsObjectives` _array_element))
    (if (and (not _completed_2) _eilmimateenemyobjective)
      (if (not (!= (`KismetArrayLibrary.Array_Length` (`self.EnemyActorArray`)) 0))
        (bind _output_get (set `self.EnemyActorArray` _actortoeliminate)))
      (`KismetArrayLibrary.Array_RemoveItem` _output_get Actor)
      (`|VariableSetRef` _array_element (make `/Game/Main/BP/GameCollection/GameQuest/S_QuestsObjectives` _names false (`self.EnemyActorArray`) _chesttoopen _eilmimateenemyobjective _ischestobjective))
      (if (== (`KismetArrayLibrary.Array_Length` (`self.EnemyActorArray`)) 0)
        (`|VariableSetRef` _array_element (make `/Game/Main/BP/GameCollection/GameQuest/S_QuestsObjectives` _names true _ _chesttoopen _eilmimateenemyobjective _ischestobjective))
        (`/Game/Main/BP/Widget/QuestsWidget/WI_QuestsPlayerDisplay.DisplayCompletedObjectives` (`self.CurrentQuests`) _array_element)
        (`self.ObjectiveCompleted`)
        (`self.BackToCommander`)
        (bind (_names_2 _completed_3 _actortoeliminate_2 _chesttoopen_2 _eilmimateenemyobjective_2 _ischestobjective_2) (break `/Game/Main/BP/GameCollection/GameQuest/S_QuestsObjectives` _array_element))
        (set `self.TempCheck` (make `/Game/Main/BP/GameCollection/GameQuest/S_QuestsObjectives` _names_2 true _actortoeliminate_2 _chesttoopen_2 _eilmimateenemyobjective_2 _ischestobjective_2))
        (`KismetArrayLibrary.Array_Remove` _questsobjective _array_index)
        (`KismetArrayLibrary.Array_Add` _questsobjective (`self.TempCheck`))))))

(event `ChestOpen`
  (params (`Chest Open Objective` :type "Actor Object Reference"))
  (bind (_activequests_questname _activequests_desrciption _activequests_secondary _activequests_completed _activequests_questsobjective) (break `/Game/Main/BP/GameCollection/GameQuest/S_QuestsDetails` (`self.ActiveQuests`)))
  (bind (_questname _desrciption _secondary _completed _questsobjective) (break `/Game/Main/BP/GameCollection/GameQuest/S_QuestsDetails` (`self.ActiveQuests`)))
  (for (_array_element _array_index) _activequests_questsobjective
    (bind (_names _completed_2 _actortoeliminate _chesttoopen _eilmimateenemyobjective _ischestobjective) (break `/Game/Main/BP/GameCollection/GameQuest/S_QuestsObjectives` _array_element))
    (if (and (== `Chest Open Objective` _chesttoopen) _ischestobjective)
      (`|VariableSetRef` _array_element (make `/Game/Main/BP/GameCollection/GameQuest/S_QuestsObjectives` _names true _actortoeliminate _chesttoopen _eilmimateenemyobjective _ischestobjective))
      (`/Game/Main/BP/Widget/QuestsWidget/WI_QuestsPlayerDisplay.DisplayCompletedObjectives` (`self.CurrentQuests`) _array_element)
      (`self.ObjectiveCompleted`)
      (bind (_names_2 _completed_3 _actortoeliminate_2 _chesttoopen_2 _eilmimateenemyobjective_2 _ischestobjective_2) (break `/Game/Main/BP/GameCollection/GameQuest/S_QuestsObjectives` _array_element))
      (set `self.TempCheck` (make `/Game/Main/BP/GameCollection/GameQuest/S_QuestsObjectives` _names_2 true _actortoeliminate_2 _chesttoopen_2 _eilmimateenemyobjective_2 _ischestobjective_2))
      (`KismetArrayLibrary.Array_Remove` _questsobjective _array_index)
      (`KismetArrayLibrary.Array_Add` _questsobjective (`self.TempCheck`)))))

(event `Completed`
  (params (Quest :type "/Game/Main/BP/GameCollection/GameQuest/S_QuestsDetails Structure"))
  (switch `name` (`.QuestName_2_8B7AC8D1444E5309F85DA7B43D78A7CE` (break `/Game/Main/BP/GameCollection/GameQuest/S_QuestsDetails` Quest))
    (:`Teasure Master`
      (set `self.Temp1QuestsCompleted` true))
    (:`HuntDown`
      (set `self.Temp2QuestsCompleted` true))
    (:`Friend in Need`
      (set `self.Temp3QuestsCompleted` true))))

(event `ObjectiveCompleted`
  (bind _objectivescompleted (`self.ObjectivesCompleted`))
  (bind (_activequests_questname _activequests_desrciption _activequests_secondary _activequests_completed _activequests_questsobjective) (break `/Game/Main/BP/GameCollection/GameQuest/S_QuestsDetails` (`self.ActiveQuests`)))
  (bind _activequests (`self.ActiveQuests`))
  (`/Engine/EditorBlueprintResources/StandardMacros.IncrementInt` _objectivescompleted
    (:`  `
      (if (>= _objectivescompleted (`KismetArrayLibrary.Array_Length` _activequests_questsobjective))
        (`/Game/Main/BP/Widget/QuestsWidget/WI_QuestsPlayerDisplay.QuestsEndMessage` (`self.CurrentQuests`) _activequests)
        (`self.QuestsMarkermaker` false)
        (`self.Completed` _activequests)
        (set `self.ActiveQuests` (struct))
        (set `self.ObjectivesCompleted` 0)
        (if (and (`self.Temp1QuestsCompleted`) (`self.Temp2QuestsCompleted`))
          (set `self.Temp3Questsactive` true))))))

(event `QuestsMarkermaker`
  (params (Ison :type Boolean))
  (bind _activequests_questname (break `/Game/Main/BP/GameCollection/GameQuest/S_QuestsDetails` (`self.ActiveQuests`)))
  (switch `name` _activequests_questname
    (:`Teasure Master`
      (`/Engine/EditorBlueprintResources/StandardMacros.IsValid` (`self.ChestMarkerRef`)
        (:`Is Valid`
          _)
        (:`Is Not Valid`
          (bind _returnvalue (`GameplayStatics.GetActorOfClass` "/Game/Main/BP/Misc/Marker/BP_MarkerChestFind.BP_MarkerChestFind_C"))
          (set `self.ChestMarkerRef` _returnvalue)))
      (message `/Game/Main/BP/Interface/Marker/BPI_Marker.QuestsMission` (`self.ChestMarkerRef`) Ison "None")
      (`KismetSystemLibrary.Delay` 1.5)
      (bind _returnvalue_2 (`GameplayStatics.GetActorOfClass` "/Game/Main/BP/Misc/Marker/BP_MarkerCommander.BP_MarkerCommander_C"))
      (`/Game/Main/BP/Misc/Marker/BP_Marker.QuestsMission` _returnvalue_2 true "None"))
    (:`HuntDown`
      (`/Engine/EditorBlueprintResources/StandardMacros.IsValid` (`self.EnemyMarkerRef`)
        (:`Is Valid`
          _)
        (:`Is Not Valid`
          (bind _returnvalue_3 (`GameplayStatics.GetActorOfClass` "/Game/Main/BP/Misc/Marker/BP_MarkerEnemyArea.BP_MarkerEnemyArea_C"))
          (set `self.EnemyMarkerRef` _returnvalue_3)))
      (message `/Game/Main/BP/Interface/Marker/BPI_Marker.QuestsMission` (`self.EnemyMarkerRef`) Ison "None")
      (`KismetSystemLibrary.Delay` 1.5)
      (bind _returnvalue_4 (`GameplayStatics.GetActorOfClass` "/Game/Main/BP/Misc/Marker/BP_MarkerCommander.BP_MarkerCommander_C"))
      (`/Game/Main/BP/Misc/Marker/BP_Marker.QuestsMission` _returnvalue_4 true "None"))
    (:`Friend in Need`
      (`/Engine/EditorBlueprintResources/StandardMacros.IsValid` (`self.FriendMarker`)
        (:`Is Valid`
          _)
        (:`Is Not Valid`
          (bind _returnvalue_5 (`GameplayStatics.GetActorOfClass` "/Game/Main/BP/Misc/Marker/BP_MarkerFriend.BP_MarkerFriend_C"))
          (bind _output_get (set `self.FriendMarker` _returnvalue_5))))
      (message `/Game/Main/BP/Interface/Marker/BPI_Marker.QuestsMission` (`self.FriendMarker`) Ison "None")
      (`/Engine/EditorBlueprintResources/StandardMacros.DoOnce` false
        (:`Completed`
          (bind _returnvalue_6 (`GameplayStatics.GetActorOfClass` "/Game/Main/BP/MainCharacter/MissionCarrier/BP_MainMission.BP_MainMission_C"))
          (`/Game/Main/BP/MainCharacter/MissionCarrier/BP_MainMission.FriendActive` _returnvalue_6 false)
          (bind _returnvalue_7 (`GameplayStatics.GetActorOfClass` "/Game/Main/BP/MainCharacter/Boss/BP_BossCall.BP_BossCall_C"))
          (set `/Game/Main/BP/MainCharacter/Boss/BP_BossCall.markerHide` _output_get _returnvalue_7)
          (`/Game/Main/BP/MainCharacter/Boss/BP_BossCall.ActiveCollision` _returnvalue_7 true))))))

(event `BackToCommander`
  (bind _returnvalue (`GameplayStatics.GetActorOfClass` "/Game/Main/BP/Misc/Marker/BP_MarkerCommander.BP_MarkerCommander_C"))
  (`/Game/Main/BP/Misc/Marker/BP_Marker.QuestsMission` _returnvalue true "None"))

(fn `LastQuestActive`
  (params (IsActive :type Boolean))
  (returns (IsActive1 :type Boolean))
  (return IsActive))