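; Player stats component for BP_AssassinPlayer that tracks health, stamina, shield, XP, level and potion counts.
; On BeginPlay it caches the owner, initializes part of the HUD and passes the player reference to components listed in ComponentCollection.
; Stat functions update values and push them to PlayerHud, while input actions consume health and shield potions.
; Reaching max XP levels up with sound and Niagara effects, discarding surplus XP.
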(event `self.ReceiveBeginPlay`
  (bind _asbp_assassin_player (cast `/Game/Main/BP/MainCharacter/Player/BP_AssassinPlayer` (`self.GetOwner`))
    (:`then`
      ;[1 1 1] Main Load Owner
      (bind _output_get (set `self.BPAssassinPlayerRef` _asbp_assassin_player))
      (`|ExecutionSequence`
        (:`then_0`
          (`KismetSystemLibrary.Delay` 0.15)
          (`/Game/Main/BP/Widget/Player/BP_PlayerWidget.increaseXP` (`/Game/Main/BP/MainCharacter/Player/BP_AssassinPlayer.PlayerHud` (`self.BPAssassinPlayerRef`)) (`self.XP`) (`self.MaxXP`))
          (`/Game/Main/BP/Widget/Player/BP_PlayerWidget.IncreaseLevel` (`/Game/Main/BP/MainCharacter/Player/BP_AssassinPlayer.PlayerHud` (`self.BPAssassinPlayerRef`)) (`self.PlayerLevel`))
          (`/Game/Main/BP/Widget/Player/BP_PlayerWidget.CollectHealth` (`/Game/Main/BP/MainCharacter/Player/BP_AssassinPlayer.PlayerHud` (`self.BPAssassinPlayerRef`)) (`self.HealthPotion`)))
        (:`then_1`
          (for _array_element (`self.Component Collection`)
            (message `/Game/Main/BP/Interface/ComponentCommunication/BPI_Components.PlayerRef` (`Actor.GetComponentByClass` (`self.GetOwner`) _array_element) _output_get)))))
    (:`CastFailed`
      (`KismetSystemLibrary.PrintString` (`KismetStringLibrary.Concat_StrStr` (`KismetSystemLibrary.GetDisplayName` self) ": can not find player Big issue.")))))

(event `ResetXP`
  (`KismetSystemLibrary.Delay` 0.25)
  (`/Game/Main/BP/Widget/Player/BP_PlayerWidget.increaseXP` (`/Game/Main/BP/MainCharacter/Player/BP_AssassinPlayer.PlayerHud` (`self.BPAssassinPlayerRef`)) (`self.XP`) (`self.MaxXP`)))

(event `EnhancedInput|/Game/Main/BP/Input/InputCollection/IA_Health`
  (params (ActionValue :type Boolean) (ElapsedSeconds :type "Float (double-precision)") (TriggeredSeconds :type "Float (double-precision)") (InputAction :type "InputAction Object Reference" :default "/Game/Main/BP/Input/InputCollection/IA_Health.IA_Health"))
  (:`Started`
    (if (and (< (`self.CurrentHealth`) 80.0) (> (`self.HealthPotion`) 0))
      (set `self.HealthPotion` (- (`self.HealthPotion`) 1))
      (`/Game/Main/BP/Widget/Player/BP_PlayerWidget.CollectHealth` (`/Game/Main/BP/MainCharacter/Player/BP_AssassinPlayer.PlayerHud` (`self.BPAssassinPlayerRef`)) (`self.HealthPotion`))
      (`self.IncreaseHealth` 100.0)
      (else
        (`/Game/Main/BP/Widget/Player/BP_PlayerWidget.CollectHealth` (`/Game/Main/BP/MainCharacter/Player/BP_AssassinPlayer.PlayerHud` (`self.BPAssassinPlayerRef`)) (`self.HealthPotion`))))))

(event `EnhancedInput|/Game/Main/BP/Input/InputCollection/IA_Shield`
  (params (ActionValue :type Boolean) (ElapsedSeconds :type "Float (double-precision)") (TriggeredSeconds :type "Float (double-precision)") (InputAction :type "InputAction Object Reference" :default "/Game/Main/BP/Input/InputCollection/IA_Shield.IA_Shield"))
  (bind _shieldpotion (`self.ShieldPotion`))
  (:`Started`
    (if (`self.ShieldCondition`)
      (bind _output_get (set `self.ShieldPotion` (- _shieldpotion 1)))
      (`/Game/Main/BP/Widget/Player/BP_PlayerWidget.CollectShieldPotion` (`/Game/Main/BP/MainCharacter/Player/BP_AssassinPlayer.PlayerHud` (`self.BPAssassinPlayerRef`)) _output_get)
      (`self.IncreaseShieldHealth` 100.0)
      (else
        (`/Game/Main/BP/Widget/Player/BP_PlayerWidget.CollectShieldPotion` (`/Game/Main/BP/MainCharacter/Player/BP_AssassinPlayer.PlayerHud` (`self.BPAssassinPlayerRef`)) _shieldpotion)))))

(fn `DeacreaseHealthCollectStore`)

(fn `DecreaseHealth`
  (params (Damage :type "Float (double-precision)"))
  (returns (IsDeath :type Boolean))
  (bind _currenthealth (`self.CurrentHealth`))
  (if (not (<= (`self.CurrentHealth`) 0.0))
    (set `self.CurrentHealth` (`KismetMathLibrary.FClamp` (- _currenthealth Damage) 0.0 (`self.MaxHealth`)))
    (if (<= _currenthealth 0.0)
      _
      (else
        (`/Game/Main/BP/Widget/Player/BP_PlayerWidget.HealthBarProgress` (`/Game/Main/BP/MainCharacter/Player/BP_AssassinPlayer.PlayerHud` (`self.BPAssassinPlayerRef`)) (`self.CurrentHealth`) (`self.MaxHealth`))
        (return false))))
  (`/Game/Main/BP/Widget/Player/BP_PlayerWidget.HealthBarProgress` (`/Game/Main/BP/MainCharacter/Player/BP_AssassinPlayer.PlayerHud` (`self.BPAssassinPlayerRef`)) 0.0 (`self.MaxHealth`))
  (return true))

(fn `DecreaseShieldHealth`
  (params (Damage :type "Float (double-precision)"))
  (returns (IsDeath :type Boolean))
  (bind _shieldhealth (`self.ShieldHealth`))
  (if (not (<= (`self.ShieldHealth`) 0.0))
    (set `self.ShieldHealth` (`KismetMathLibrary.FClamp` (- _shieldhealth Damage) 0.0 (`self.MaxShieldHealth`)))
    (if (<= _shieldhealth 0.0)
      _
      (else
        (`/Game/Main/BP/Widget/Player/BP_PlayerWidget.ShieldBarProgress` (`/Game/Main/BP/MainCharacter/Player/BP_AssassinPlayer.PlayerHud` (`self.BPAssassinPlayerRef`)) (`self.ShieldHealth`) (`self.MaxShieldHealth`))
        (return false))))
  (`/Game/Main/BP/Widget/Player/BP_PlayerWidget.ShieldBarProgress` (`/Game/Main/BP/MainCharacter/Player/BP_AssassinPlayer.PlayerHud` (`self.BPAssassinPlayerRef`)) 0.0 (`self.MaxShieldHealth`))
  (return true))

(fn `DecreaseStamina`
  (params (DecreaseStamina :type "Float (double-precision)"))
  (returns (`No stamina` :type Boolean))
  (bind _maxstamina (`self.MaxStamina`))
  (if (not (<= (`self.CurrentStamina`) 0.0))
    (set `self.CurrentStamina` (`KismetMathLibrary.FClamp` (- (`self.CurrentStamina`) DecreaseStamina) 0.0 (`self.MaxStamina`)))
    (if (<= (`self.CurrentStamina`) 0.0)
      _
      (else
        (`/Game/Main/BP/Widget/Player/BP_PlayerWidget.StaminaProgress` (`/Game/Main/BP/MainCharacter/Player/BP_AssassinPlayer.PlayerHud` (`self.BPAssassinPlayerRef`)) (`self.CurrentStamina`) _maxstamina)
        (return false))))
  (`/Game/Main/BP/Widget/Player/BP_PlayerWidget.StaminaProgress` (`/Game/Main/BP/MainCharacter/Player/BP_AssassinPlayer.PlayerHud` (`self.BPAssassinPlayerRef`)) 0.0 _maxstamina)
  (return true))

(fn `HealthCollectableIncrease`
  (bind _output_get (set `self.HealthPotion` (`KismetMathLibrary.Clamp` (+ (`self.HealthPotion`) 1) 0 10)))
  (`/Game/Main/BP/Widget/Player/BP_PlayerWidget.CollectHealth` (`/Game/Main/BP/MainCharacter/Player/BP_AssassinPlayer.PlayerHud` (`self.BPAssassinPlayerRef`)) _output_get))

(fn `IncreaseHealth`
  (params (Increase :type "Float (double-precision)"))
  (bind _output_get (set `self.CurrentHealth` (`KismetMathLibrary.FClamp` (+ (`self.CurrentHealth`) Increase) 0.0 (`self.MaxHealth`))))
  (`/Game/Main/BP/Widget/Player/BP_PlayerWidget.HealthBarProgress` (`/Game/Main/BP/MainCharacter/Player/BP_AssassinPlayer.PlayerHud` (`self.BPAssassinPlayerRef`)) _output_get (`self.MaxHealth`)))

(fn `IncreaseLevel`
  (params (IncreaseLevel :type Integer))
  (bind _bpassassinplayerref (`self.BPAssassinPlayerRef`))
  (bind _bpassassinplayerref_2 (`self.BPAssassinPlayerRef`))
  (bind _output_get (set `self.PlayerLevel` (+ (`self.PlayerLevel`) IncreaseLevel)))
  (set `self.MaxXP` (+ (`self.MaxXP`) 150.0))
  (set `self.XP` 0.0)
  (`GameplayStatics.SpawnSoundAtLocation` "/Game/Main/Misc/audio/Hit/epic-level-up.epic-level-up" (`Actor.K2_GetActorLocation` _bpassassinplayerref) (struct) 1.0 1.0 0.0 null null)
  (`/Game/Main/BP/Widget/Player/BP_PlayerWidget.IncreaseLevel` (`/Game/Main/BP/MainCharacter/Player/BP_AssassinPlayer.PlayerHud` _bpassassinplayerref) _output_get)
  (`/Game/Main/BP/Widget/Player/BP_PlayerWidget.Increase LevelUpdates` (`/Game/Main/BP/MainCharacter/Player/BP_AssassinPlayer.PlayerHud` _bpassassinplayerref_2) (`KismetTextLibrary.Conv_IntToText` (`self.PlayerLevel`)))
  (`self.ResetXP`)
  (`NiagaraFunctionLibrary.SpawnSystemAtLocation` "/Game/Main/Niagara/NS_Achieve.NS_Achieve" (`SceneComponent.K2_GetComponentLocation` (`/Game/Main/BP/MainCharacter/Player/BP_AssassinPlayer.SpawnEmitter` _bpassassinplayerref_2))))

(fn `IncreaseMaxHealth`
  (params (Increase :type "Float (double-precision)"))
  (bind _output_get (set `self.MaxHealth` (+ (`self.MaxHealth`) Increase)))
  (`/Game/Main/BP/Widget/Player/BP_PlayerWidget.HealthBarProgress` (`/Game/Main/BP/MainCharacter/Player/BP_AssassinPlayer.PlayerHud` (`self.BPAssassinPlayerRef`)) (`self.CurrentHealth`) _output_get))

(fn `IncreaseMaxShieldHealth`
  (params (ShieldMax :type "Float (double-precision)"))
  (bind _output_get (set `self.MaxShieldHealth` (+ (`self.MaxHealth`) ShieldMax)))
  (`/Game/Main/BP/Widget/Player/BP_PlayerWidget.ShieldBarProgress` (`/Game/Main/BP/MainCharacter/Player/BP_AssassinPlayer.PlayerHud` (`self.BPAssassinPlayerRef`)) (`self.ShieldHealth`) _output_get))

(fn `IncreaseMaxStamina`
  (params (stamina :type "Float (double-precision)"))
  (bind _output_get (set `self.MaxStamina` (+ (`self.MaxStamina`) stamina)))
  (`/Game/Main/BP/Widget/Player/BP_PlayerWidget.StaminaProgress` (`/Game/Main/BP/MainCharacter/Player/BP_AssassinPlayer.PlayerHud` (`self.BPAssassinPlayerRef`)) (`self.CurrentStamina`) _output_get))

(fn `IncreaseShieldHealth`
  (params (Damage :type "Float (double-precision)"))
  (bind _maxshieldhealth (`self.MaxShieldHealth`))
  (bind _output_get (set `self.ShieldHealth` (`KismetMathLibrary.FClamp` (+ (`self.ShieldHealth`) Damage) 0.0 _maxshieldhealth)))
  (`/Game/Main/BP/Widget/Player/BP_PlayerWidget.ShieldBarProgress` (`/Game/Main/BP/MainCharacter/Player/BP_AssassinPlayer.PlayerHud` (`self.BPAssassinPlayerRef`)) _output_get _maxshieldhealth))

(fn `IncreaseStamina`
  (params (Stamina :type "Float (double-precision)"))
  (returns (StaminaMax :type Boolean))
  (bind _maxstamina (`self.MaxStamina`))
  (bind _output_get (set `self.CurrentStamina` (`KismetMathLibrary.FClamp` (+ (`self.CurrentStamina`) Stamina) 0.0 _maxstamina)))
  (`/Game/Main/BP/Widget/Player/BP_PlayerWidget.StaminaProgress` (`/Game/Main/BP/MainCharacter/Player/BP_AssassinPlayer.PlayerHud` (`self.BPAssassinPlayerRef`)) _output_get _maxstamina)
  (if (>= (`self.CurrentStamina`) _maxstamina)
    (return false)))

(fn `IncreaseXP`
  (params (XP :type "Float (double-precision)"))
  (bind _maxxp (`self.MaxXP`))
  (bind _output_get (set `self.XP` (+ (`self.XP`) XP)))
  (`/Game/Main/BP/Widget/Player/BP_PlayerWidget.increaseXP` (`/Game/Main/BP/MainCharacter/Player/BP_AssassinPlayer.PlayerHud` (`self.BPAssassinPlayerRef`)) _output_get _maxxp)
  ;[1 1 1] if the extra xp value is lose then it cheats the player
  (if (>= (`self.XP`) _maxxp)
    (`self.IncreaseLevel` 1)))

(fn `ShieldCollectableIncrease`
  (bind _output_get (set `self.ShieldPotion` (`KismetMathLibrary.Clamp` (+ (`self.ShieldPotion`) 1) 0 10)))
  (`/Game/Main/BP/Widget/Player/BP_PlayerWidget.CollectShieldPotion` (`/Game/Main/BP/MainCharacter/Player/BP_AssassinPlayer.PlayerHud` (`self.BPAssassinPlayerRef`)) _output_get))