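; Climb system component for the assassin player, an unfinished draft: BeginPlay and GrabWall are empty and the logic chains are never triggered.
; One unwired chain lazily caches the owning player and calls GrabWall.
; The other line-traces forward from pelvis and head sockets; when both hit, it switches movement to Flying, slides the capsule off the wall surface facing it, and clears Climb.
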(event `self.ReceiveBeginPlay`)

(event `EnhancedInput|/Game/Main/BP/Input/InputCollection/IA_Climb`
  (params (ActionValue :type Boolean) (ElapsedSeconds :type "Float (double-precision)") (TriggeredSeconds :type "Float (double-precision)") (InputAction :type "InputAction Object Reference" :default "/Game/Main/BP/Input/InputCollection/IA_Climb.IA_Climb")))

(event `Grab Wall`)