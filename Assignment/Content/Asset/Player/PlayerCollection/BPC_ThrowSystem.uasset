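; Player component for aiming and throwing distraction rocks, with a predicted arc preview, available when no bow is held.
; While aiming, a looping timer predicts the projectile path, rebuilds it as spline meshes and eases camera pitch toward the landing point.
; Mouse Y adjusts throw strength within limits.
; Attack plays a montage whose notify spawns the rock with the predicted velocity and decrements the rock count, with movement disabled until blend-out.
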(event `/Game/Main/BP/Interface/ComponentCommunication/BPI_Components.PlayerRef`
  (params (PlayerRef :type "/Game/Main/BP/MainCharacter/Player/BP_AssassinPlayer Object Reference"))
  (bind _player_ref (`self.Player Ref`))
  (bind _output_get (set `self.Player Ref` PlayerRef))
  (set `self.CameraRef` (`/Game/Main/BP/MainCharacter/Player/BP_AssassinPlayer.FollowCamera` _output_get))
  (set `self.ThrowLocationRef` (`/Game/Main/BP/MainCharacter/Player/BP_AssassinPlayer.ThrowArrowStart` _player_ref))
  (set `self.SplineRef` (`/Game/Main/BP/MainCharacter/Player/BP_AssassinPlayer.RockSpline` _player_ref)))

(event `EnhancedInput|/Game/Main/BP/Input/InputCollection/IA_Aim`
  (params (ActionValue :type Boolean) (ElapsedSeconds :type "Float (double-precision)") (TriggeredSeconds :type "Float (double-precision)") (InputAction :type "InputAction Object Reference" :default "/Game/Main/BP/Input/InputCollection/IA_Aim.IA_Aim"))
  (:`Started`
    (if (not (`/Game/Main/BP/MainCharacter/Player/PlayerCollection/BPC_PlayerAttack.HasBow` (`/Game/Main/BP/MainCharacter/Player/BP_AssassinPlayer.BPC_PlayerAttack` (`self.Player Ref`))))
      (`self.AimThrow`)))
  (:`Completed`
    (`self.StopAimRock`)))

(event `AimThrow`
  (`self.ThrowTrace`)
  (`self.ChangeRotationSeed`))

(event `InputAxisKey|MouseY`
  (params (AxisValue :type "Float (single-precision)"))
  (`self.AimDistance_Mouse` AxisValue))

(event `StopAimRock`
  (`self.ThrowTraceStop`)
  (`self.revertrotationseed`))

(event `ThrowTraceStop`
  ;[1 1 1] AimThrwoingPath
  (`KismetSystemLibrary.K2_ClearAndInvalidateTimerHandle` (`self.Throw_TraceTH`))
  (`self.DeleteSplinePoints`))

(event `ThrowTrace`
  ;[1 1 1] AimThrwoingPath
  (bind _returnvalue (`KismetSystemLibrary.K2_SetTimerDelegate` (delegate `ThrowTraceTimer`) 0.02 true))
  (set `self.Throw_TraceTH` _returnvalue))

(event `ThrowTraceTimer`
  ;[1 1 1] AimThrwoingPath
  (`self.DeleteSplinePoints`)
  (bind (_outpathpositions _distance _location) (`self.RockTrajectory`))
  (set `self.Rock_TraceLocations` _outpathpositions)
  (set `self.ThrowRockFar` (> _distance 1500.0))
  (`self.ThrowRock_PitchTowardsTarget` _location)
  (`self.DrawSpline`))

(event `ChangeRotationSeed`
  ;[0.06076 0.06076 0.06076] All Changes When entering Aim Mode
  (set `self.Rock_Aiming` true))

(event `revertrotationseed`
  ;[0.06076 0.06076 0.06076] All Changes When entering Aim Mode
  (set `self.Rock_Aiming` false))

(event `EnhancedInput|/Game/Main/BP/Input/InputCollection/IA_Attack`
  (params (ActionValue :type Boolean) (ElapsedSeconds :type "Float (double-precision)") (TriggeredSeconds :type "Float (double-precision)") (InputAction :type "InputAction Object Reference" :default "/Game/Main/BP/Input/InputCollection/IA_Attack.IA_Attack"))
  (:`Started`
    (`self.ThrowRock`)))

(event `ThrowRock`
  (bind _returnvalue (`GameplayStatics.GetPlayerCharacter` 0))
  (bind _returnvalue_2 (`GameplayStatics.GetPlayerCharacter` 0))
  (bind _rock_aiming (`self.Rock_Aiming`))
  (if _rock_aiming
    (if (> (`self.Rocks`) 0)
      (`CharacterMovementComponent.DisableMovement` (`Character.CharacterMovement` _returnvalue_2))
      (`|PlayMontage` (`Character.Mesh` _returnvalue_2) (`self.ThrowM`)
        (:`OnBlendOut`
          (if (`self.Rock_Aiming`)
            (`self.ThrowTrace`))
          (`/Engine/EditorBlueprintResources/StandardMacros.IsValid` _returnvalue
            (:`Is Valid`
              (`CharacterMovementComponent.SetMovementMode` (`Character.CharacterMovement` _returnvalue) "MOVE_Walking" 0))))
        (:`OnNotifyBegin`
          (`self.SpawnRock`)
          (`self.ThrowTraceStop`)))
      (else
        (`KismetSystemLibrary.PrintString` (select `bool` _rock_aiming :`false` "FIRST Aim" :`true` "Out of Rocks - find and pick up a rock to use this function.") true true (struct :`R` 1.0 :`G` 0.062048 :`A` 1.0) 5.0 :!label _label)))
    (else
      (goto _label))))

(event `SpawnRock`
  (bind _player_ref (`self.Player Ref`))
  (bind _returnvalue (`SceneComponent.K2_GetComponentToWorld` (`/Game/Main/BP/MainCharacter/Player/BP_AssassinPlayer.Throwables` _player_ref)))
  (`KismetSystemLibrary.Delay` 0.1)
  (bind _returnvalue_2 (`|SpawnActorFromClass` (`/Game/Main/BP/MainCharacter/Player/BP_AssassinPlayer.ThrowDistractObject` _player_ref) (`KismetMathLibrary.MakeTransform` (.location _returnvalue) (`KismetMathLibrary.MakeRotator` (.roll (.rotation _returnvalue)) (.pitch (.rotation _returnvalue)) (.yaw (.rotation _returnvalue)))) "AdjustIfPossibleButAlwaysSpawn" "MultiplyWithRoot" null null))
  (set `self.Rock_Ref` _returnvalue_2)
  (set `MovementComponent.Velocity` (`self.Rock_Velocity`) (`/Game/Main/BP/Throw/BP_ThrowStone.ProjectileMovement` _returnvalue_2))
  (`/Engine/EditorBlueprintResources/StandardMacros.DecrementInt` (`self.Rocks`)))

(fn `AddSplineComp`
  (params (Owner :type "Actor Object Reference"))
  (returns (ReturnValue :type "SplineMeshComponent Object Reference"))
  (bind _returnvalue (`|AddComponentByClass` :`self` Owner :`Class` "/Script/Engine.SplineMeshComponent" :`bManualAttachment` true))
  (`SceneComponent.SetMobility` _returnvalue "Movable")
  (`PrimitiveComponent.SetMaterial` _returnvalue 0 "/Game/StealthSystem/Materials/Throw_Spline_Mat.Throw_Spline_Mat")
  (`StaticMeshComponent.SetStaticMesh` _returnvalue "/Engine/BasicShapes/Cylinder.Cylinder")
  (`SplineMeshComponent.SetForwardAxis` _returnvalue "Z" true)
  (`PrimitiveComponent.SetCollisionEnabled` _returnvalue "NoCollision")
  (return _returnvalue))

(fn `AimDistance_Mouse`
  (params (A :type "Float (double-precision)"))
  (bind _returnvalue (`KismetMathLibrary.FInterpTo` (`self.Rock_Direction`) (+ (`self.Rock_Direction`) (* A 1.3)) (`GameplayStatics.GetWorldDeltaSeconds`) 1.0))
  (if (`self.Rock_Aiming`)
    (if (and (> _returnvalue -0.5) (< _returnvalue 0.9))
      (set `self.Rock_Direction` _returnvalue))))

(fn `DeleteSplinePoints`
  (bind _rock_splinemeshes (`self.Rock_SplineMeshes`))
  (message `/Game/Main/BP/Interface/ComponentCommunication/BPI_Components.StealthInterface_DeleteSplines` (`self.GetOwner`) _rock_splinemeshes)
  (`KismetArrayLibrary.Array_Clear` _rock_splinemeshes)
  (`SplineComponent.ClearSplinePoints` (`self.SplineRef`) true))

(fn `DrawSpline`
  (bind _rock_tracelocations (`self.Rock_TraceLocations`))
  (bind _splineref (`self.SplineRef`))
  (bind _splineref_2 (`self.SplineRef`))
  (bind _returnvalue (- (`SplineComponent.GetNumberOfSplinePoints` (`self.SplineRef`)) 2))
  (for _array_element _rock_tracelocations
    (`SplineComponent.AddSplinePoint` _splineref _array_element "World" true))
  (`SplineComponent.SetSplinePointType` _splineref (`KismetArrayLibrary.Array_LastIndex` _rock_tracelocations) "CurveClamped" true)
  (for _index (range (+ _returnvalue 1))
    (bind _returnvalue_2 (`self.AddSplineComp` (`self.GetOwner`)))
    (bind _returnvalue_3 (`KismetSystemLibrary.MakeLiteralDouble` (`KismetMathLibrary.Lerp` 0.02 0.025 (/ (`KismetMathLibrary.Conv_IntToDouble` _index) (`KismetMathLibrary.Conv_IntToDouble` _returnvalue)))))
    (bind _returnvalue_4 (`KismetMathLibrary.MakeVector2D` _returnvalue_3 _returnvalue_3))
    (`SplineMeshComponent.SetStartScale` _returnvalue_2 _returnvalue_4 true)
    (`SplineMeshComponent.SetEndScale` _returnvalue_2 (/ _returnvalue_4 1.0) true)
    (`KismetArrayLibrary.Array_Add` (`self.Rock_SplineMeshes`) _returnvalue_2)
    (bind _returnvalue_5 (+ _index 1))
    (`SplineMeshComponent.SetStartAndEnd` _returnvalue_2 (`|GetArrayItem` (`self.Rock_TraceLocations`) _index) (`SplineComponent.GetTangentAtSplinePoint` _splineref_2 _index "World") (`|GetArrayItem` (`self.Rock_TraceLocations`) _returnvalue_5) (`SplineComponent.GetTangentAtSplinePoint` _splineref_2 _returnvalue_5 "World") true)))

(fn `RockTrajectory`
  (returns (OutPathPositions :type "Array of Vector Structure") (Distance :type "Float (single-precision)") (Location :type "Vector Structure"))
  (bind _throwlocationref (`self.ThrowLocationRef`))
  (bind _rock_direction (`self.Rock_Direction`))
  (bind _returnvalue (`KismetMathLibrary.GetForwardVector` (`SceneComponent.K2_GetComponentRotation` _throwlocationref)))
  (bind _output_get (set `self.Rock_Velocity` (* (+ _returnvalue (* _returnvalue _rock_direction)) (`self.Rock Projectile Speed`))))
  (bind (_outhit _outpathpositions) (`GameplayStatics.Blueprint_PredictProjectilePath_ByTraceChannel` (+ (`SceneComponent.K2_GetComponentLocation` _throwlocationref) _returnvalue) _output_get true 10.0 "ECC_Visibility" false (`|MakeArray` null :!type "Actor Object Reference") "None" 1.0 (`KismetMathLibrary.Lerp` 3.0 14.0 (+ _rock_direction 0.5))))
  (bind (_bblockinghit _binitialoverlap _time _distance _location) (`GameplayStatics.BreakHitResult` _outhit))
  (return _outpathpositions _distance _location))

(fn `StealthInterface_DeleteSplines`
  (params (Spline :type "Array of SplineMeshComponent Object Reference (by ref)"))
  (return))

(fn `ThrowRock_PitchTowardsTarget`
  (params (Location :type "Vector Structure"))
  (bind _returnvalue (`GameplayStatics.GetPlayerCharacter` 0))
  (bind _returnvalue_2 (`Pawn.GetController` _returnvalue))
  (bind _returnvalue_3 (`Controller.GetControlRotation` _returnvalue_2))
  (bind (_returnvalue_roll _returnvalue_pitch _returnvalue_yaw) (`KismetMathLibrary.BreakRotator` (`KismetMathLibrary.FindLookAtRotation` (`SceneComponent.K2_GetComponentLocation` (`self.CameraRef`)) Location)))
  (`/Engine/EditorBlueprintResources/StandardMacros.IsValid` _returnvalue
    (:`Is Valid`
      (`/Engine/EditorBlueprintResources/StandardMacros.IsValid` _returnvalue_2
        (:`Is Valid`
          (`Controller.SetControlRotation` _returnvalue_2 (`KismetMathLibrary.MakeRotator` (.roll _returnvalue_3) (.pitch (`KismetMathLibrary.RInterpTo` _returnvalue_3 (`KismetMathLibrary.MakeRotator` _returnvalue_roll _returnvalue_pitch _returnvalue_yaw) (`GameplayStatics.GetWorldDeltaSeconds`) 7.0)) (.yaw _returnvalue_3))))))))