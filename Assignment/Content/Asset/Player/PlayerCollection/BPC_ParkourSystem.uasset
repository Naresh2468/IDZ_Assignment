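; Parkour component for the assassin player that provides vaulting and floor sliding.
; Vaulting runs stepped sphere traces to find an obstacle's start, depth and landing, then plays a depth-chosen or random montage in Flying mode with Motion Warping targets.
; Sliding starts above a speed threshold, swaps the capsule and uses looping timers and floor-normal checks to align, continue or end it.
; A ceiling trace toggles crouch.
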(event `SprintSlide`
  (bind _bp_assassin_player (`self.BP Assassin Player`))
  (if (> (`KismetMathLibrary.VSize` (`MovementComponent.Velocity` (`Character.CharacterMovement` (`self.BP Assassin Player`)))) 200.0) :!label _label
    (set `SpringArmComponent.bDoCollisionTest` false (`/Game/Main/BP/MainCharacter/Player/BP_AssassinPlayer.CameraArm` (`self.BP Assassin Player`)))
    (if (not (and (`AnimInstance.Montage_IsPlaying` (`SkeletalMeshComponent.GetAnimInstance` (`Character.Mesh` _bp_assassin_player)) null) (`NavMovementComponent.IsFalling` (`Character.CharacterMovement` _bp_assassin_player))))
      (`|ExecutionSequence`
        (:`then_0`
          (set `self.isSlide?` true)
          (`AnimInstance.Montage_Play` (`SkeletalMeshComponent.GetAnimInstance` (`Character.Mesh` (`self.BP Assassin Player`))) (`self.BeginSlide`) 1.0 "MontageLength" 0.0 true))
        (:`then_1`
          (`/Game/Main/BP/MainCharacter/Player/BP_AssassinPlayer.SlideCapusle` (`self.BP Assassin Player`) true))
        (:`then_2`
          (bind _returnvalue (`KismetSystemLibrary.K2_SetTimerDelegate` (`|CreateDelegate` :!event `Trace Floor while Slide`) 0.01 true))
          (set `self.SlideTimerHandle` _returnvalue))))))

(event `/Game/Main/BP/Interface/ComponentCommunication/BPI_Components.PlayerRef`
  (params (PlayerRef :type "/Game/Main/BP/MainCharacter/Player/BP_AssassinPlayer Object Reference"))
  (bind _output_get (set `self.BP Assassin Player` PlayerRef))
  (`/Engine/EditorBlueprintResources/StandardMacros.IsValid` _output_get
    (:`Is Valid`
      (`KismetSystemLibrary.PrintString` "Pakour System"))))

(event `Trace Floor while Slide`
  (bind _continueslidehandle (`self.ContinueSlideHandle`))
  (bind _bp_assassin_player (`self.BP Assassin Player`))
  (`|ExecutionSequence`
    (:`then_0`
      (`self.CheckifOnFloor` 4.0)
      (`KismetSystemLibrary.K2_ClearAndInvalidateTimerHandle` (`self.SlideTimerHandle`))
      (if (`KismetSystemLibrary.K2_IsValidTimerHandle` _continueslidehandle)
        (`KismetSystemLibrary.K2_ClearAndInvalidateTimerHandle` _continueslidehandle))
      (`/Game/Main/BP/MainCharacter/Player/BP_AssassinPlayer.SlideCapusle` _bp_assassin_player false)
      (`/Game/Main/BP/MainCharacter/Player/BP_AssassinPlayer.SlideResetXYRotation` _bp_assassin_player)
      (set `SpringArmComponent.bDoCollisionTest` true (`/Game/Main/BP/MainCharacter/Player/BP_AssassinPlayer.CameraArm` _bp_assassin_player)))
    (:`then_1`
      (`self.Align The Player Floor` 5.0))
    (:`then_2`
      (`self.CheckHitSurface` 0.0 20.0 80.0 "ForDuration")
      (`KismetSystemLibrary.K2_ClearAndInvalidateTimerHandle` (`self.SlideTimerHandle`)))))

(event `Key|X`
  (params (Key :type "Key Structure"))
  (:`Pressed`
    (goto _label)))

(event `CheckShouldSildeContinue`
  (bind _slidetimerhandle (`self.SlideTimerHandle`))
  (bind _bp_assassin_player (`self.BP Assassin Player`))
  (if (`self.isSlide?`)
    (if (`.isSlopeUp` (`self.SlideCurrentFloorAngleAndDirection`))
      (set `MovementComponent.Velocity` (`self.CurrentSlideVelocity`) (`Character.CharacterMovement` (`self.BP Assassin Player`)))
      (bind _returnvalue (`KismetSystemLibrary.K2_SetTimerDelegate` (`|CreateDelegate` :!event `ContinueSliding`) 0.001 true))
      (set `self.ContinueSlideHandle` _returnvalue)
      (set `self.CurrentAngle` (`self.SlideCurrentFloorAngleAndDirection`))
      (else
        (`AnimInstance.Montage_Play` (`SkeletalMeshComponent.GetAnimInstance` (`Character.Mesh` (`self.BP Assassin Player`))) (`self.SlideEnd`) 1.0 "MontageLength" 0.0 true :!label _label_2)
        (`KismetSystemLibrary.RetriggerableDelay` 0.02)
        (`|ExecutionSequence`
          (:`then_0`
            (if (`KismetSystemLibrary.K2_IsValidTimerHandle` _slidetimerhandle)
              (`KismetSystemLibrary.K2_ClearAndInvalidateTimerHandle` _slidetimerhandle)))
          (:`then_1`
            (`/Game/Main/BP/MainCharacter/Player/BP_AssassinPlayer.SlideCapusle` _bp_assassin_player false))
          (:`then_2`
            (`/Game/Main/BP/MainCharacter/Player/BP_AssassinPlayer.SlideResetXYRotation` _bp_assassin_player)
            (set `SpringArmComponent.bDoCollisionTest` true (`/Game/Main/BP/MainCharacter/Player/BP_AssassinPlayer.CameraArm` (`self.BP Assassin Player`)))))))))

(event `PlayGetupFromSlide`
  (goto _label_2))

(event `ContinueSliding`
  (bind _angle (`self.SlideCurrentFloorAngleAndDirection`))
  (bind _bp_assassin_player (`self.BP Assassin Player`))
  (bind (_returnvalue_roll _returnvalue_pitch _returnvalue_yaw) (`KismetMathLibrary.BreakRotator` (`Actor.K2_GetActorRotation` _bp_assassin_player)))
  (bind _charactermovement (`Character.CharacterMovement` _bp_assassin_player))
  (bind _output_get (set `self.CurrentAngle` _angle))
  (if (< (`KismetMathLibrary.FInterpTo` _output_get _angle (`GameplayStatics.GetWorldDeltaSeconds`) 0.4) 3.0)
    (if (< (`KismetMathLibrary.VSize` (`MovementComponent.Velocity` (`Character.CharacterMovement` (`self.BP Assassin Player`)))) (`self.Speed toStopSlide`))
      (`KismetSystemLibrary.K2_ClearAndInvalidateTimerHandle` (`self.ContinueSlideHandle`) :!label _label_3)
      (`self.PlayGetupFromSlide`))
    (else
      (`|ExecutionSequence`
        (:`then_0`
          (`Pawn.AddMovementInput` _bp_assassin_player (`KismetMathLibrary.GetForwardVector` (`KismetMathLibrary.MakeRotator` 0.0 0.0 _returnvalue_yaw)) 1.0 false)
          (set `CharacterMovementComponent.MaxWalkSpeed` 1500.0 _charactermovement)
          (set `CharacterMovementComponent.MaxAcceleration` 500.0 _charactermovement))
        (:`then_1`
          (`self.CheckHitSurface` 0.0)
          (goto _label_3))))))

(event `TraceCeiling`
  (bind _bp_assassin_player (`self.BP Assassin Player`))
  (bind _returnvalue (+ (`Actor.K2_GetActorLocation` (`self.BP Assassin Player`)) (0.0 0.0 70.0)))
  (bind (_outhit _returnvalue_2) (`KismetSystemLibrary.CapsuleTraceSingle` _returnvalue _returnvalue 34.0 50.0 "TraceTypeQuery1" false (`|MakeArray` null :!type "Actor Object Reference")))
  (if _returnvalue_2
    (`AnimInstance.Montage_Stop` (`SkeletalMeshComponent.GetAnimInstance` (`Character.Mesh` _bp_assassin_player)) 0.2 null)
    (if (not (`/Game/Main/BP/MainCharacter/Player/BP_AssassinPlayer.Crouched` _bp_assassin_player))
      (`/Game/Main/BP/MainCharacter/Player/BP_AssassinPlayer.Crouch State` _bp_assassin_player)
      (set `self.TraceCeling` true))
    (elif (`/Game/Main/BP/MainCharacter/Player/BP_AssassinPlayer.Crouched` _bp_assassin_player)
      (`/Game/Main/BP/MainCharacter/Player/BP_AssassinPlayer.Crouch State` _bp_assassin_player)
      (set `self.TraceCeling` false))))

(event `VaultSystem`
  (bind _returnvalue (`KismetMathLibrary.VSize` (`MovementComponent.Velocity` (`Character.CharacterMovement` (`self.BP Assassin Player`)))))
  (`KismetSystemLibrary.PrintString` (`KismetStringLibrary.Conv_DoubleToString` _returnvalue) :!label _label_4)
  (if (and (> _returnvalue 300.0) (not (`NavMovementComponent.IsFalling` (`Character.CharacterMovement` (`self.BP Assassin Player`)))))
    (bind (_vaultstart _vaultmiddle _vaultland _vaultdistanceloc) (`self.VaultTraceF` 380.0 100.0 45.0 100.0))
    (if (`self.CanVault`)
      (`self.Vault` _vaultstart _vaultmiddle _vaultland _vaultdistanceloc))))

(event `EnhancedInput|/Game/Main/BP/Input/InputCollection/IA_Vault`
  (params (ActionValue :type Boolean) (ElapsedSeconds :type "Float (double-precision)") (TriggeredSeconds :type "Float (double-precision)") (InputAction :type "InputAction Object Reference" :default "/Game/Main/BP/Input/InputCollection/IA_Vault.IA_Vault"))
  (:`Started`
    (goto _label_4)))

(fn `SlideCurrentFloorAngleAndDirection`
  (returns (Angle :type "Float (double-precision)") (isSlopeUp :type Boolean))
  (bind _bp_assassin_player (`self.BP Assassin Player`))
  (bind (_currentfloor_bblockinghit _currentfloor_bwalkablefloor _currentfloor_blinetrace _currentfloor_floordist _currentfloor_linedist _currentfloor_hitresult) (break `FindFloorResult` (`CharacterMovementComponent.CurrentFloor` (`Character.CharacterMovement` _bp_assassin_player))))
  (bind (_bblockinghit _binitialoverlap _time _distance _location _impactpoint _normal) (`GameplayStatics.BreakHitResult` _currentfloor_hitresult))
  (bind (_returnvalue_roll _returnvalue_pitch) (`KismetMathLibrary.BreakRotator` (`KismetMathLibrary.MakeRotFromXY` _normal (`Actor.GetActorForwardVector` _bp_assassin_player))))
  (return (`KismetMathLibrary.DegAcos` (`KismetMathLibrary.Dot_VectorVector` _normal (0.0 0.0 1.0))) (> (* _returnvalue_roll _returnvalue_pitch) 0.0)))

(fn `VaultTraceF`
  (params (InitialTrace :type "Float (double-precision)") (`SecondaryTraceZ offset` :type "Float (double-precision)") (SecondaryTraceGap :type "Float (double-precision)") (LandingPositionfowardoffset :type "Float (double-precision)"))
  (returns (VaultStart :type "Vector Structure") (VaultMiddle :type "Vector Structure") (VaultLand :type "Vector Structure") (VaultDistanceLoc :type Integer))
  (locals (`Vault Start` :type "Vector Structure" :default (0.0 0.0 0.0)) (`Vault Middle` :type "Vector Structure" :default (0.0 0.0 0.0)) (`Vault Land` :type "Vector Structure" :default (0.0 0.0 0.0)))
  (bind _bp_assassin_player (`self.BP Assassin Player`))
  ;[1 1 1] Do  Line trace to trace for object to vault ovr.if the object found ,the function run continues to fin the target location ,vault distance is set to 0 so it can be incremented to find the vaulting distance
  (for _index (range 4)
    (bind _returnvalue (+ (`Actor.K2_GetActorLocation` _bp_assassin_player) (`KismetMathLibrary.MakeVector` 0.0 0.0 (* _index 30))))
    (bind (_outhit _returnvalue_2) (`KismetSystemLibrary.SphereTraceSingle` :`Start` _returnvalue :`End` (+ _returnvalue (* (`KismetMathLibrary.GetForwardVector` (`Actor.K2_GetActorRotation` _bp_assassin_player)) 180.0)) :`Radius` 6.0 :`TraceChannel` "TraceTypeQuery1" :`DrawDebugType` "ForDuration"))
    (if _returnvalue_2
      (`|ExecutionSequence`
        (:`then_0`
          (break))
        (:`then_1`
          (set `self.VaultDistance` 0)
          ;[1 1 1] Length of the Object Calculate
          (for _index_2 (range 11)
            (`/Engine/EditorBlueprintResources/StandardMacros.IncrementInt` (`self.VaultDistance`)
              (:`  `
                (bind _returnvalue_3 (+ (`.Location` (`GameplayStatics.BreakHitResult` _outhit)) (* (`Actor.GetActorForwardVector` (`self.BP Assassin Player`)) _index_2 (`local.SecondaryTraceGap`))))
                (bind (_outhit_2 _returnvalue_4) (`KismetSystemLibrary.SphereTraceSingle` :`Start` (+ _returnvalue_3 (`KismetMathLibrary.MakeVector` 0.0 0.0 (`local.SecondaryTraceZ offset`))) :`End` _returnvalue_3 :`Radius` 10.0 :`TraceChannel` "TraceTypeQuery1" :`DrawDebugType` "ForDuration"))
                (if _returnvalue_4
                  ;[1 1 1] if the first / initial trace the vault starting location is set and sphere trace is used to check if there is anything to block then vault is cancel.
                  (if (== _index_2 0)
                    (bind (_bblockinghit _binitialoverlap _time _distance _location _impactpoint _normal _impactnormal _physmat _hitactor _hitcomponent _hitbonename _bonename _hititem _elementindex _faceindex _tracestart _traceend) (`GameplayStatics.BreakHitResult` _outhit_2))
                    (bind _output_get (set `local.Vault Start` _impactpoint))
                    (bind _returnvalue_5 (+ _output_get (0.0 0.0 20.0)))
                    (bind (_outhit_3 _returnvalue_6) (`KismetSystemLibrary.SphereTraceSingle` :`Start` _returnvalue_5 :`End` _returnvalue_5 :`Radius` 10.0 :`TraceChannel` "TraceTypeQuery1" :`DrawDebugType` "ForDuration"))
                    (if _returnvalue_6
                      (set `self.CanVault` false)
                      (break)))
                  (else
                    ;[1 1 1] Find the landing location to by doing line trace downward from an offset so it not  directly down to the Object but to the floor
                    (set `self.CanVault` true)
                    (`|ExecutionSequence`
                      (:`then_0`
                        (bind _returnvalue_7 (+ _traceend (`Actor.GetActorForwardVector` (`self.BP Assassin Player`))))
                        (bind _outhit_4 (`KismetSystemLibrary.LineTraceSingle` :`Start` _returnvalue_7 :`End` (- _returnvalue_7 (0.0 0.0 100.0)) :`TraceChannel` "TraceTypeQuery1" :`DrawDebugType` "ForDuration"))
                        (bind (_outhit_5 _returnvalue_8) (`KismetSystemLibrary.SphereTraceSingle` :`Start` _returnvalue_7 :`End` _returnvalue_7 :`Radius` 20.0 :`TraceChannel` "TraceTypeQuery1" :`DrawDebugType` "ForDuration"))
                        (set `self.Land` _returnvalue_7)
                        (if _returnvalue_8
                          (set `self.CanVault` false)))
                      (:`then_1`
                        (break))))))))
          (return (`local.Vault Start`) (`local.Vault Middle`) (`local.Vault Land`) (`self.VaultDistance`)))))))