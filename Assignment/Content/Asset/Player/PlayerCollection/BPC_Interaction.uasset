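; Player interaction component that handles weapon pickups, chests, quest and mission givers, rideable animals, doors and collectables.
; On IA_Interact, DetectItem sphere-traces from the player's SwimEnter point along the camera's forward vector.
; It dispatches the hit by actor tag or interface message, adding weapons and chest contents to the equipment system.
; Collectables play a montage, with separate events to attach them to the hand socket and destroy them.
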(event `/Game/Main/BP/Interface/ComponentCommunication/BPI_Components.PlayerRef`
  (params (PlayerRef :type "/Game/Main/BP/MainCharacter/Player/BP_AssassinPlayer Object Reference"))
  (set `self.BP Assassin PlayerRef` PlayerRef))

(event `EnhancedInput|/Game/Main/BP/Input/InputCollection/IA_Interact`
  (params (ActionValue :type Boolean) (ElapsedSeconds :type "Float (double-precision)") (TriggeredSeconds :type "Float (double-precision)") (InputAction :type "InputAction Object Reference" :default "/Game/Main/BP/Input/InputCollection/IA_Interact.IA_Interact"))
  (:`Started`
    (`self.DetectItem`)))

(event `CollectItem`
  (`|PlayMontage` (`Character.Mesh` (`self.BP Assassin PlayerRef`)) (`self.CollectM`)))

(event `StartCollect`
  (message `/Game/Main/BP/Interface/ComponentCommunication/BPI_Collectables.CollectHand` (`self.Collectable`) (`Character.Mesh` (`self.BP Assassin PlayerRef`)) "CollectHand"))

(event `DestroryCollectable`
  (message `/Game/Main/BP/Interface/ComponentCommunication/BPI_Collectables.DestroyCollectables` (`self.Collectable`))
  (set `self.Collectable` null))

(fn `DetectItem`
  (bind _bp_assassin_playerref (`self.BP Assassin PlayerRef`))
  (bind _bpc_equipmentsystem (`/Game/Main/BP/MainCharacter/Player/BP_AssassinPlayer.BPC_EquipmentSystem` (`self.BP Assassin PlayerRef`)))
  (bind _returnvalue (`SceneComponent.K2_GetComponentLocation` (`/Game/Main/BP/MainCharacter/Player/BP_AssassinPlayer.SwimEnter` _bp_assassin_playerref)))
  (bind (_outhit _returnvalue_2) (`KismetSystemLibrary.SphereTraceSingleForObjects` _returnvalue (+ _returnvalue (* (`KismetMathLibrary.GetForwardVector` (`SceneComponent.K2_GetComponentRotation` (`/Game/Main/BP/MainCharacter/Player/BP_AssassinPlayer.FollowCamera` _bp_assassin_playerref))) 400.0)) 40.0 (`|MakeArray` "ObjectTypeQuery2" :!type "EObjectTypeQuery Enum")))
  (if _returnvalue_2
    (`|ExecutionSequence`
      (:`then_0`
        (bind (_bblockinghit _binitialoverlap _time _distance _location _impactpoint _normal _impactnormal _physmat _hitactor) (`GameplayStatics.BreakHitResult` _outhit))
        (if (`Actor.ActorHasTag` _hitactor "Items")
          (bind _asbp_weapon_master (cast `/Game/Main/BP/GameCollection/EquipementSystem/Weapon/BP_WeaponMaster` _hitactor))
          ;[1 1 1] EquippedSystem
          (`/Game/Main/BP/GameCollection/EquipementSystem/DataCollection/BPC_EquipmentSystem.AddWeapon` _bpc_equipmentsystem (`/Game/Main/BP/GameCollection/EquipementSystem/Weapon/BP_WeaponMaster.Item` _asbp_weapon_master))
          (`Actor.K2_DestroyActor` _asbp_weapon_master)))
      (:`then_1`
        (if (`KismetSystemLibrary.DoesImplementInterface` _hitactor "/Game/Main/BP/Interface/BPI_QuestsCommunicate.BPI_QuestsCommunicate_C")
          (bind _item (message `/Game/Main/BP/Interface/BPI_QuestsCommunicate.OpenChest` _hitactor))
          (`/Game/Main/BP/GameCollection/EquipementSystem/DataCollection/BPC_EquipmentSystem.AddWeapon` _bpc_equipmentsystem _item)))
      (:`then_2`
        (if (`KismetSystemLibrary.DoesImplementInterface` _hitactor "/Game/Main/BP/Interface/BPI_Misc.BPI_Misc_C")
          (message `/Game/Main/BP/Interface/BPI_Misc.QuestsGiver` _hitactor)))
      (:`then_3`
        (if (`KismetSystemLibrary.DoesImplementInterface` _hitactor "/Game/Main/BP/Interface/BPI_AnimalConnection.BPI_AnimalConnection_C")
          (message `/Game/Main/BP/Interface/BPI_AnimalConnection.RideAnimals` _hitactor)))
      (:`then_4`
        (`/Engine/EditorBlueprintResources/StandardMacros.IsValid` _hitactor
          (:`Is Valid`
            (if (`Actor.ActorHasTag` _hitactor "Collect")
              (set `self.Collectable` _hitactor)
              (`self.CollectItem`)))))
      (:`then_5`
        (`/Engine/EditorBlueprintResources/StandardMacros.IsValid` _hitactor
          (:`Is Valid`
            (if (`KismetSystemLibrary.DoesImplementInterface` _hitactor "/Game/Main/BP/Interface/BPI_Misc.BPI_Misc_C")
              (message `/Game/Main/BP/Interface/BPI_Misc.DoorToggle` _hitactor)))))
      (:`then_6`
        (`/Engine/EditorBlueprintResources/StandardMacros.IsValid` _hitactor
          (:`Is Valid`
            (if (`KismetSystemLibrary.DoesImplementInterface` _hitactor "/Game/Main/BP/Interface/BPI_Misc.BPI_Misc_C")
              (message `/Game/Main/BP/Interface/BPI_Misc.MissionGiver` _hitactor))))))))