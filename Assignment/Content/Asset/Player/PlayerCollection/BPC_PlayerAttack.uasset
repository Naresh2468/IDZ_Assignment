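; Player combat component for the assassin character, handling sword combos, shield blocking and bow-and-arrow shooting from input actions.
; Sword attacks buffer the next input to chain staged montages, briefly turning the player toward control rotation.
; Timer-driven sphere traces damage "Damageable" actors with shake, sound and particles.
; The bow spawns an arrow while aiming, times the draw for launch strength, aims by camera trace and updates ammo UI.
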(event `self.PlayerRef`
  (params (PlayerRef :type "Object Object Reference"))
  (bind (_output_get _output_get_2) (set `self.BP Assassin Player` null PlayerRef))
  (set `self.InitialField Of View` (`CameraComponent.FieldOfView` (`/Game/Asset/Player/PlayerCollection/BPC_PlayerAttack.FollowCamera` _output_get_2)))
  (set `self.InititalOffset` (`SpringArmComponent.SocketOffset` (`/Game/Asset/Player/PlayerCollection/BPC_PlayerAttack.CameraArm` _output_get_2))))

(event `EnhancedInput|`
  (params (ActionValue :type Boolean) (ElapsedSeconds :type "Float (double-precision)") (TriggeredSeconds :type "Float (double-precision)"))
  (bind (_bp_assassin_player _bp_assassin_player_2) (`self.BP Assassin Player`))
  (bind (_bp_assassin_player_3 _bp_assassin_player_4) (`self.BP Assassin Player`))
  (bind (_bp_assassin_player_5 _bp_assassin_player_6) (`self.BP Assassin Player`))
  (bind _mesh (`Character.Mesh` _bp_assassin_player_6))
  ;[0.05729 0.05729 0.05729] Shield Blocking
  (:`Started`
    (if (`self.EquippedShield`)
      (`/Engine/EditorBlueprintResources/StandardMacros.FlipFlop`
        (:`A`
          (`self.CheckTheShieldEquipped`
            (:`true`
              (set `/Game/Asset/Player/PlayerCollection/BPC_PlayerAttack.IsBlocking?` true _bp_assassin_player_6)
              (`|PlayMontage` _mesh
                (:`OnNotifyBegin`
                  (`SceneComponent.K2_AttachToComponent` (`/Game/Asset/Player/PlayerCollection/BPC_PlayerAttack.BackShieldHolster/HandToggle` _bp_assassin_player_2) (`Character.Mesh` _bp_assassin_player_2) (`self.ShieldBoneName`) "KeepRelative" "KeepRelative" "KeepRelative" true)
                  (set `/Game/Asset/Player/PlayerCollection/BPC_PlayerAttack.Sprinting` (`self.ShieldOnHandPlayerSpeed`) (`.BP Assassin Player` (`self.BP Assassin Player`))))))))
        (:`B`
          (`self.CheckTheShieldEquipped`
            (:`true`
              (set `/Game/Asset/Player/PlayerCollection/BPC_PlayerAttack.IsBlocking?` false _bp_assassin_player_6)
              (`|PlayMontage` _mesh
                (:`OnNotifyBegin`
                  (`SceneComponent.K2_AttachToComponent` (`/Game/Asset/Player/PlayerCollection/BPC_PlayerAttack.BackShieldHolster/HandToggle` _bp_assassin_player_4) (`Character.Mesh` _bp_assassin_player_4) "ShieldHolster" "KeepRelative" "KeepRelative" "KeepRelative" true)
                  (set `/Game/Asset/Player/PlayerCollection/BPC_PlayerAttack.Sprinting` (`self.PlayerNomralSpeed`) (`.BP Assassin Player` (`self.BP Assassin Player`)))))))))
      (`self.EquipShield` (`/Game/Asset/Player/PlayerCollection/BPC_PlayerAttack.PlayerHud` (`.BP Assassin Player` (`self.BP Assassin Player`))) (`/Game/Asset/Player/PlayerCollection/BPC_PlayerAttack.IsBlocking?` _bp_assassin_player_6)))))

(event `EnhancedInput|`
  (params (ActionValue :type Boolean) (ElapsedSeconds :type "Float (double-precision)") (TriggeredSeconds :type "Float (double-precision)"))
  ;[0.05729 0.05729 0.05729] AttackAction
  (:`Started`
    (if (not (`/Game/Asset/Player/PlayerCollection/BPC_PlayerAttack.Crouched` (`.BP Assassin Player` (`self.BP Assassin Player`))))
      (if (`self.CanAttack?`)
        (`self.SwordAttack`)
        (`self.AttackRotationInstanct`)
        (`KismetSystemLibrary.Delay` 0.3)
        (`KismetSystemLibrary.K2_ClearAndInvalidateTimerHandle` (`self.RotationAttack`))))))

(event `EnhancedInput|`
  (params (ActionValue :type Boolean) (ElapsedSeconds :type "Float (double-precision)") (TriggeredSeconds :type "Float (double-precision)"))
  (bind (_bp_assassin_player _bp_assassin_player_2) (`self.BP Assassin Player`))
  (bind _swordholster (`/Game/Asset/Player/PlayerCollection/BPC_PlayerAttack.SwordHolster` _bp_assassin_player_2))
  (bind _equippedweapon (`/Game/Asset/Player/PlayerCollection/BPC_PlayerAttack.EquippedWeapon` _bp_assassin_player_2))
  (bind _returnvalue (`SkeletalMeshComponent.GetAnimInstance` (`Character.Mesh` _bp_assassin_player_2)))
  (:`Started`
    (if (`self.EquippedSword?`)
      (if (not (`self.CanAttack?`))
        (bind _output_get (set `self.CanAttack?` true))
        (message `/Game/Asset/Player/PlayerCollection/BPC_PlayerAttack.EquipSword` _returnvalue _output_get)
        (`SceneComponent.SetVisibility` _swordholster false false)
        (`SceneComponent.SetVisibility` _equippedweapon _output_get false)
        (else
          (bind _output_get_2 (set `self.CanAttack?` false))
          (message `/Game/Asset/Player/PlayerCollection/BPC_PlayerAttack.EquipSword` _returnvalue _output_get_2)
          (`SceneComponent.SetVisibility` _swordholster true false)
          (`SceneComponent.SetVisibility` _equippedweapon _output_get_2 false)))
      (`self.EquipSwordUI` (`/Game/Asset/Player/PlayerCollection/BPC_PlayerAttack.PlayerHud` (`.BP Assassin Player` (`self.BP Assassin Player`))) (`self.CanAttack?`)))))

(event `SwordAttack`
  ;[0.05729 0.05729 0.05729] SowrdAttack
  (if (`self.isAttacking`)
    (set `self.SaveAttack` true)
    (else
      (set `self.isAttacking` true)
      ;[0.05729 0.05729 0.05729] AttackStage
      (switch `int` (`self.Attackindex`) :!label _label
        (:`0`
          (`self.Attack_1`))
        (:`1`
          (`self.Attack_2`))
        (:`2`
          (`self.Attack_3`))
        (:`3`
          (`self.Attack_4`))))))

(event `Attack_1`
  ;[0.05729 0.05729 0.05729] AttackStage
  (`/Engine/EditorBlueprintResources/StandardMacros.DoOnce` false :!label _label_2
    (:`Completed`
      (`KismetSystemLibrary.Delay` (`self.DelayGap`))
      (`|PlayMontage` (`Character.Mesh` (`.BP Assassin Player` (`self.BP Assassin Player`))) (`KismetArrayLibrary.Array_Random` (`self.AttackM`)) 1.25
        (:`then`
          (set `self.Attackindex` 1)
          (goto _label_2 :!via `Reset`))))))

(event `Attack_2`
  ;[0.05729 0.05729 0.05729] AttackStage
  (`/Engine/EditorBlueprintResources/StandardMacros.DoOnce` false :!label _label_3
    (:`Completed`
      (`KismetSystemLibrary.Delay` (`self.DelayGap`))
      (`|PlayMontage` (`Character.Mesh` (`.BP Assassin Player` (`self.BP Assassin Player`))) null 1.25
        (:`then`
          (set `self.Attackindex` 2)
          (goto _label_3 :!via `Reset`))))))

(event `Attack_3`
  ;[0.05729 0.05729 0.05729] AttackStage
  (`/Engine/EditorBlueprintResources/StandardMacros.DoOnce` false :!label _label_4
    (:`Completed`
      (`KismetSystemLibrary.Delay` (`self.DelayGap`))
      (`|PlayMontage` (`Character.Mesh` (`.BP Assassin Player` (`self.BP Assassin Player`))) (`KismetArrayLibrary.Array_Random` (`|MakeArray` null null :!type "AnimMontage Object Reference")) 1.25
        (:`then`
          (set `self.Attackindex` 3)
          (goto _label_4 :!via `Reset`))))))

(event `Attack_4`
  ;[0.05729 0.05729 0.05729] AttackStage
  (`/Engine/EditorBlueprintResources/StandardMacros.DoOnce` false :!label _label_5
    (:`Completed`
      (`KismetSystemLibrary.Delay` (`self.DelayGap`))
      (`|PlayMontage` (`Character.Mesh` (`.BP Assassin Player` (`self.BP Assassin Player`))) null 1.25
        (:`then`
          (set `self.Attackindex` 4)
          (goto _label_5 :!via `Reset`))))))

(event `SwordAtackCombo`
  ;[0.05729 0.05729 0.05729] SwordCombo
  (if (`self.SaveAttack`)
    (set `self.SaveAttack` false)
    (goto _label)
    (else
      (`self.stopCombo`))))

(event `StopCombo`
  ;[0.05729 0.05729 0.05729] SwordCombo
  ;;[0.05729 0.05729 0.05729] Stop
  (set `self.isAttacking` false)
  (set `self.Attackindex` 0))

(event `AttackRotationInstanct`
  ;[0.01042 0.01042 0.01042] Rotate player accroding to the mouse rotation instant while Attack
  (bind _returnvalue (`KismetSystemLibrary.K2_SetTimerDelegate` (`|CreateDelegate` :!event `Rotate`) 0.002 true))
  (set `self.RotationAttack` _returnvalue))

(event `Rotate`
  (bind (_bp_assassin_player _bp_assassin_player_2) (`self.BP Assassin Player`))
  (bind _returnvalue (`Actor.K2_GetActorRotation` _bp_assassin_player_2))
  (bind (_returnvalue_roll _returnvalue_pitch _returnvalue_yaw) (`KismetMathLibrary.BreakRotator` (`KismetMathLibrary.RInterpTo` _returnvalue (`Pawn.GetControlRotation` _bp_assassin_player_2) 0.002 (`self.RotationSpeed`))))
  ;[0.01042 0.01042 0.01042] Rotate player accroding to the mouse rotation instant while Attack
  (`Actor.K2_SetActorRotation` _bp_assassin_player_2 (`KismetMathLibrary.MakeRotator` (.roll _returnvalue) (.pitch _returnvalue) _returnvalue_yaw) false))

(event `SwordTraceLoop`
  (bind (_bp_assassin_player _bp_assassin_player_2) (`self.BP Assassin Player`))
  ;[0.05729 0.05729 0.05729] SwordTrace, Effects, Sound
  (bind (_outhit _returnvalue) (`KismetSystemLibrary.SphereTraceSingle` :`Start` (`SceneComponent.K2_GetComponentLocation` (`/Game/Asset/Player/PlayerCollection/BPC_PlayerAttack.TopPoints` _bp_assassin_player_2)) :`End` (`SceneComponent.K2_GetComponentLocation` (`/Game/Asset/Player/PlayerCollection/BPC_PlayerAttack.BottomPoints` _bp_assassin_player_2)) :`Radius` 10.0 :`TraceChannel` "TraceTypeQuery1" :`DrawDebugType` "ForDuration" :`TraceColor` (struct :`R` 1.0 :`G` 0.211286 :`B` 0.951492 :`A` 1.0) :`DrawTime` 0.2))
  (if _returnvalue
    (bind (_bblockinghit _binitialoverlap _time _distance _location _impactpoint _normal _impactnormal _physmat _hitactor) (`GameplayStatics.BreakHitResult` _outhit))
    (if (`Actor.ActorHasTag` _hitactor "Damageable")
      (`/Engine/EditorBlueprintResources/StandardMacros.DoOnce` false :!label _label_6
        (:`Completed`
          (`GameplayStatics.ApplyDamage` _hitactor 10.0)
          (`self.CameraShakeHit` _location)
          (`self.SwordHitSound`)
          (`GameplayStatics.SpawnEmitterAtLocation` null _location (`KismetMathLibrary.MakeRotFromXY` _normal _normal) (`KismetArrayLibrary.Array_Random` (`|MakeArray` (0.5 0.5 0.5) (0.6 0.6 0.6) (0.4 0.4 0.4) :!type "Vector Structure")))
          (`KismetSystemLibrary.PrintString` (`KismetSystemLibrary.GetDisplayName` _hitactor))
          (`|ExecutionSequence`
            (:`then_0`
              (`KismetSystemLibrary.Delay` 0.5)
              (goto _label_6 :!via `Reset`))
            (:`then_1`
              (if (`KismetSystemLibrary.DoesImplementInterface` _hitactor)
                (message `/Game/Asset/Player/PlayerCollection/BPC_PlayerAttack.Destruction` _hitactor))))))
      (else
        (`/Engine/EditorBlueprintResources/StandardMacros.DoOnce` false :!label _label_7
          (:`Completed`
            (`GameplayStatics.PlaySoundAtLocation` null (`Actor.K2_GetActorLocation` (`.BP Assassin Player` (`self.BP Assassin Player`))) (struct) 1.0 1.0 0.0 null null null null)))))))

(event `ResetSoundHit`
  ;[0.05729 0.05729 0.05729] SwordTrace, Effects, Sound
  (goto _label_7 :!via `Reset`))

(event `StartSwordTrace`
  ;[0.05729 0.05729 0.05729] SwordTrace, Effects, Sound
  (bind _returnvalue (`KismetSystemLibrary.K2_SetTimerDelegate` (`|CreateDelegate` :!event `SwordTraceLoop`) 0.008 true))
  (set `self.SowrdTraceTimer` _returnvalue))

(event `PushDabKickTrace`
  ;[0.05729 0.05729 0.05729] SwordTrace, Effects, Sound
  (`self.Push Dab Kick Tracep`))

(event `Stop Sword trace`
  ;[0.05729 0.05729 0.05729] SwordTrace, Effects, Sound
  (`self.SwordTraceStop`))

(event `SwordHitSound`
  ;[0.05729 0.05729 0.05729] SwordTrace, Effects, Sound
  (`GameplayStatics.PlaySoundAtLocation` null (`Actor.K2_GetActorLocation` (`.BP Assassin Player` (`self.BP Assassin Player`))) (struct) 1.0 1.0 0.0 null null null null))

(event `CameraShakeHit`
  (params (Epicenter :type "Vector Structure"))
  ;[0.05729 0.05729 0.05729] SwordTrace, Effects, Sound
  (`GameplayStatics.PlayWorldCameraShake` null Epicenter 0.0 2000.0))

(event `EnhancedInput|`
  (params (ActionValue :type Boolean) (ElapsedSeconds :type "Float (double-precision)") (TriggeredSeconds :type "Float (double-precision)"))
  (bind (_bp_assassin_player _bp_assassin_player_2) (`self.BP Assassin Player`))
  (bind _hasbow (`self.HasBow`))
  ;[0.05729 0.05729 0.05729] BowAndArrow
  (:`Started`
    (if _hasbow
      (`self.AimBeginEndToggle` true)
      (`self.AimCameraToggle` _bp_assassin_player_2 true)))
  (:`Completed`
    (if _hasbow
      (`self.AimBeginEndToggle` false)
      (`self.AimCameraToggle` _bp_assassin_player_2 false))))

(event `DrawArrowBegin`
  ;[0.05729 0.05729 0.05729] BowAndArrow
  ;;[0.7656 0.7241 0.2965] DrawArrow
  (`self.DrawArrowB`))

(event `DrawIncrementTime`
  ;[0.05729 0.05729 0.05729] BowAndArrow
  ;;[0.7656 0.7241 0.2965] DrawArrow
  (`self.DrawTimeP`))

(event `EnhancedInput|`
  (params (ActionValue :type Boolean) (ElapsedSeconds :type "Float (double-precision)") (TriggeredSeconds :type "Float (double-precision)"))
  ;[0.05729 0.05729 0.05729] BowAndArrow
  (:`Started`
    (`self.EquipBowProcess`)))

(event `DrawArrowEnd`
  ;[0.05729 0.05729 0.05729] BowAndArrow
  ;;[0.7656 0.7241 0.2965] DrawArrow
  (`self.DrawArrowE`))

(event `AimBeginEndToggle`
  (params (BowAimming :type Boolean))
  ;[0.05729 0.05729 0.05729] BowAndArrow
  (`self.AimTogglep` BowAimming))

(event `FireArrowBegin`
  (params (Direction :type "Vector Structure") (HitActor :type Boolean))
  (bind _bowandarrowcurrent (`self.BowAndArrowCurrent`))
  ;[0.05729 0.05729 0.05729] BowAndArrow
  ;;[0.7656 0.7241 0.2965] FireArrow
  (if (`self.isDrawingArrow`)
    (set `self.IsFireArrow` true)
    (set `self.ShootArrowFire` true)
    (set `self.FireArrowSecond` null)
    (`self.LaunchArrow` Direction HitActor)
    (if (> _bowandarrowcurrent 0)
      (bind _result (`/Engine/EditorBlueprintResources/StandardMacros.DecrementInt` _bowandarrowcurrent)
        (:`  `
          (`self.CurrentArrow` (`.BowArrowWidget` (`self.BowArrowWidget`)) _result)
          (`self.DrawArrowEnd`)
          (`|PlayMontage` (`Character.Mesh` (`.BP Assassin Player` (`self.BP Assassin Player`))) (`self.FireBowM`)
            (:`OnCompleted`
              _)
            (:`OnInterrupted`
              _))
          (`self.FireArrowEnd`))))))

(event `EnhancedInput|`
  (params (ActionValue :type Boolean) (ElapsedSeconds :type "Float (double-precision)") (TriggeredSeconds :type "Float (double-precision)"))
  (bind _hasbow (`self.HasBow`))
  ;[0.05729 0.05729 0.05729] BowAndArrow
  (:`Started`
    (if _hasbow
      (`self.DrawArrowBegin`)))
  (:`Completed`
    (if _hasbow
      (bind (_returnvalue _bblockinghit) (`self.Calculate AIMDirection` (`.BP Assassin Player` (`self.BP Assassin Player`))))
      (`self.FireArrowBegin` _returnvalue _bblockinghit))))

(event `FireArrowEnd`
  ;[0.05729 0.05729 0.05729] BowAndArrow
  ;;[0.7656 0.7241 0.2965] FireArrow
  (`self.FireArrowE`))

(event `Key|NumPadNine`
  (params (Key :type "Key Structure"))
  ;[1 1 1] ARROW sLOW motion Process
  ;;[1 1 1] Debug Arrow Follow
)

(fn `AimTogglep`
  (params (BowAimming :type Boolean))
  (bind _output_get (set `self.BowAimming` BowAimming))
  (if _output_get
    (if (> (`self.BowAndArrowCurrent`) 0)
      (`self.SpawnArrow`)
      (else
        (`self.DrawArrowEnd` :!label _label)
        (`self.DestroyArrow`)
        (set `self.BowAimming` false)))
    (else
      (goto _label))))

(fn `Calculate AIMDirection`
  (returns (ReturnValue :type "Vector Structure") (bBlockingHit :type Boolean))
  (bind _followcamera (`/Game/Asset/Player/PlayerCollection/BPC_PlayerAttack.FollowCamera` (`.BP Assassin Player` (`self.BP Assassin Player`))))
  (bind _returnvalue (`SceneComponent.K2_GetComponentLocation` _followcamera))
  (bind _outhit (`KismetSystemLibrary.LineTraceSingle` :`Start` _returnvalue :`End` (+ _returnvalue (* (`SceneComponent.GetForwardVector` _followcamera) 1000.0)) :`TraceChannel` "TraceTypeQuery1" :`DrawDebugType` "ForDuration" :`TraceColor` (struct :`R` 0.035066 :`G` 0.269265 :`B` 1.0 :`A` 1.0)))
  (bind (_arrowref _arrowref_2) (`self.ArrowRef`)
    (:`then`
      (bind (_bblockinghit _binitialoverlap _time _distance _location _impactpoint _normal _impactnormal _physmat _hitactor _hitcomponent _hitbonename _bonename _hititem _elementindex _faceindex _tracestart _traceend) (`GameplayStatics.BreakHitResult` _outhit))
      (return (`KismetMathLibrary.GetDirectionUnitVector` (`Actor.K2_GetActorLocation` _arrowref_2) (`KismetMathLibrary.SelectVector` _location _traceend _bblockinghit)) _bblockinghit))
    (:`else`)))

(fn `DestroyArrow`
  (bind (_arrowref _arrowref_2) (`self.ArrowRef`)
    (:`then`
      (`Actor.K2_DestroyActor` _arrowref_2))
    (:`else`)))

(fn `DrawArrowB`
  (`self.CanDrawBow`
    (:`Yes`
      (set `self.isDrawingArrow` true)
      (bind _returnvalue (`KismetSystemLibrary.K2_SetTimerDelegate` (`|CreateDelegate` :!event `DrawIncrementTime`) (`self.DrawIncrement`) true))
      (set `self.ArrowTimer` _returnvalue))
    (:`No`
      (`self.DrawArrowEnd`)
      (`self.DestroyArrow`))))

(fn `DrawArrowE`
  (set `self.isDrawingArrow` false)
  (set `self.DrawTime` 0.0)
  (`KismetSystemLibrary.K2_ClearAndInvalidateTimerHandle` (`self.ArrowTimer`))
  (`self.DestroyArrow`)
  (`self.OnDrawEnd`))

(fn `DrawTimeP`
  (bind _output_get (set `self.DrawTime` (+ (`self.DrawTime`) (`self.DrawIncrement`))))
  (`KismetSystemLibrary.PrintString` (`KismetStringLibrary.Conv_DoubleToString` _output_get))
  (`self.OnDrawOnging` 1.0 _output_get))

(fn `EquipBowProcess`
  (bind (_bp_assassin_player _bp_assassin_player_2) (`self.BP Assassin Player`))
  (bind _charactermovement (`Character.CharacterMovement` (`.BP Assassin Player` (`self.BP Assassin Player`))))
  (bind _charactermovement_2 (`Character.CharacterMovement` (`.BP Assassin Player` (`self.BP Assassin Player`))))
  (if (`self.IsEquipBow`)
    (if (not (`self.HasBow`))
      (bind _output_get (set `self.HasBow` true))
      (`self.EquipBowOnHand` _bp_assassin_player_2)
      (bind _returnvalue (`|CreateWidget` null))
      (bind (_output_get_2 _output_get_3) (set `self.BowArrowWidget` null _returnvalue))
      (`UserWidget.AddToViewport` _output_get_3 0)
      (`self.BowArrowCrosshair` _output_get_3 true)
      (set `CharacterMovementComponent.bUseControllerDesiredRotation` true _charactermovement)
      (set `CharacterMovementComponent.bOrientRotationToMovement` false _charactermovement)
      (set `CharacterMovementComponent.MaxWalkSpeed` 150.0 _charactermovement)
      (`self.EquipBow` (`/Game/Asset/Player/PlayerCollection/BPC_PlayerAttack.PlayerHud` (`.BP Assassin Player` (`self.BP Assassin Player`))) _output_get)
      (`/Engine/EditorBlueprintResources/StandardMacros.DoOnce` false
        (:`Completed`
          (bind _output_get_4 (set `self.BowAndArrowCurrent` (`self.BowAndArrowMax`)))
          (`self.CurrentArrow` (`.BowArrowWidget` (`self.BowArrowWidget`)) _output_get_4)))
      (else
        (set `self.HasBow` false)
        (`self.UnequipBowOnHand` _bp_assassin_player_2)
        (`Widget.RemoveFromParent` (`.BowArrowWidget` (`self.BowArrowWidget`)))
        (set `CharacterMovementComponent.bUseControllerDesiredRotation` false _charactermovement_2)
        (set `CharacterMovementComponent.bOrientRotationToMovement` true _charactermovement_2)
        (set `CharacterMovementComponent.MaxWalkSpeed` 300.0 _charactermovement)
        (`self.DestroyArrow`)
        (`self.EquipBow` (`/Game/Asset/Player/PlayerCollection/BPC_PlayerAttack.PlayerHud` (`.BP Assassin Player` (`self.BP Assassin Player`))) _output_get)))))

(fn `FireArrowE`
  (set `self.IsFireArrow` false)
  (if (`self.BowAimming`)
    (set `self.ShootArrowFire` false)
    (if (> (`self.BowAndArrowCurrent`) 0)
      (`self.AimBeginEndToggle` true)
      (else
        (`self.AimBeginEndToggle` false)))))

(fn `LaunchArrow`
  (params (Direction :type "Vector Structure") (HitActor :type Boolean))
  (bind (_arrowref _arrowref_2) (`self.ArrowRef`)
    (:`then`
      (set `self.FireArrowSecond` null _arrowref_2)
      (`Actor.K2_DetachFromActor` _arrowref_2 "KeepWorld" "KeepWorld" "KeepWorld")
      (`GameplayStatics.PlaySoundAtLocation` null (`Actor.K2_GetActorLocation` (`.BP Assassin Player` (`self.BP Assassin Player`))) (struct) 1.0 1.0 0.0 null null null null)
      (`self.FireArrow` _arrowref_2 Direction (`KismetMathLibrary.FClamp` (`KismetMathLibrary.NormalizeToRange` (`self.DrawTime`) 0.0 (`self.MaxDrawTIme`))) HitActor)
      (set `self.ArrowRef` null))
    (:`else`)))

(fn `Push Dab Kick Tracep`
  (bind _returnvalue (`SceneComponent.K2_GetComponentLocation` (`/Game/Asset/Player/PlayerCollection/BPC_PlayerAttack.StabPushSphereTrace` (`.BP Assassin Player` (`self.BP Assassin Player`)))))
  (bind (_outhit _returnvalue_2) (`KismetSystemLibrary.SphereTraceSingle` :`Start` _returnvalue :`End` _returnvalue :`Radius` 15.0 :`TraceChannel` "TraceTypeQuery1" :`DrawDebugType` "ForDuration" :`TraceColor` (struct :`R` 1.0 :`G` 0.211286 :`B` 0.951492 :`A` 1.0) :`DrawTime` 0.1))
  (if _returnvalue_2
    (bind (_bblockinghit _binitialoverlap _time _distance _location _impactpoint _normal _impactnormal _physmat _hitactor) (`GameplayStatics.BreakHitResult` _outhit))
    (if (`Actor.ActorHasTag` _hitactor "Damageable")
      (`GameplayStatics.ApplyDamage` _hitactor 10.0)
      (`self.CameraShakeHit` _location)
      (`GameplayStatics.SpawnEmitterAtLocation` null _location (`KismetMathLibrary.MakeRotFromXY` _normal _normal) (`KismetArrayLibrary.Array_Random` (`|MakeArray` (0.5 0.5 0.5) (0.6 0.6 0.6) (0.4 0.4 0.4) :!type "Vector Structure"))))))

(fn `SpawnArrow`
  (bind (_bp_assassin_player _bp_assassin_player_2) (`self.BP Assassin Player`))
  (bind _returnvalue (`|SpawnActorFromClass` null (`KismetMathLibrary.MakeTransform` (`Actor.K2_GetActorLocation` _bp_assassin_player_2)) "Undefined" "OverrideRootScale" null _bp_assassin_player_2))
  (bind (_output_get _output_get_2) (set `self.ArrowRef` null _returnvalue))
  (`Actor.K2_AttachToComponent` _output_get_2 (`Character.Mesh` _bp_assassin_player_2) (`self.ArrowSocketName`) "SnapToTarget" "SnapToTarget" "SnapToTarget" true))

(fn `SwordStartTraceLoop`
  (bind (_bp_assassin_player _bp_assassin_player_2) (`self.BP Assassin Player`))
  (bind (_outhit _returnvalue) (`KismetSystemLibrary.SphereTraceSingle` :`Start` (`SceneComponent.K2_GetComponentLocation` (`/Game/Asset/Player/PlayerCollection/BPC_PlayerAttack.TopPoints` _bp_assassin_player_2)) :`End` (`SceneComponent.K2_GetComponentLocation` (`/Game/Asset/Player/PlayerCollection/BPC_PlayerAttack.BottomPoints` _bp_assassin_player_2)) :`Radius` 12.0 :`TraceChannel` "TraceTypeQuery1" :`DrawDebugType` "ForDuration" :`TraceColor` (struct :`R` 1.0 :`G` 0.211286 :`B` 0.951492 :`A` 1.0) :`DrawTime` 0.1))
  (bind (_bblockinghit _binitialoverlap _time _distance _location _impactpoint _normal _impactnormal _physmat _hitactor) (`GameplayStatics.BreakHitResult` _outhit))
  (if (and _returnvalue (`Actor.ActorHasTag` _hitactor "Damageable"))
    (`/Engine/EditorBlueprintResources/StandardMacros.DoOnce` false
      (:`Completed`
        (`GameplayStatics.ApplyDamage` _hitactor 10.0)))))

(fn `SwordTraceStop`
  (`KismetSystemLibrary.K2_ClearAndInvalidateTimerHandle` (`self.SowrdTraceTimer`))
  (`self.ResetSoundHit`))